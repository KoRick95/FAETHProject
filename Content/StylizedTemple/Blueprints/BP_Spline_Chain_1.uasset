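; Spline-driven chain actor that builds a run of deformed chain meshes along an editable spline in its construction script.
; Segment length scales with actor X scale, and each whole segment gets a Z-forward spline mesh with query and physics collision.
; Tangents are clamped to segment length, and only each segment's start is nudged in X and Y.
; Any leftover spline shorter than a segment stays empty, and there is no runtime logic.
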(fn `UserConstructionScript`
  (bind _returnvalue_x (`KismetMathLibrary.BreakVector` (`self.GetActorScale3D`)))
  (bind _spline (`self.Spline`))
  (set `self.ChainSegmentLength` (* _returnvalue_x 297.0))
  (for _index (range (`KismetMathLibrary.FTrunc` (/ (`SplineComponent.GetSplineLength` (`self.Spline`)) (`self.ChainSegmentLength`))))
    (bind _returnvalue (`AddComponent|NODE_AddSplineMeshComponent-0`))
    (`StaticMeshComponent.SetStaticMesh` _returnvalue (`self.Spline Mesh`))
    (`SplineMeshComponent.SetForwardAxis` _returnvalue "Z" true)
    (`PrimitiveComponent.SetCollisionEnabled` _returnvalue "QueryAndPhysics")
    (bind _returnvalue_2 (* _index (`self.ChainSegmentLength`)))
    (bind _returnvalue_3 (* (+ _index 1) (`self.ChainSegmentLength`)))
    (`SplineMeshComponent.SetStartAndEnd` _returnvalue (`KismetMathLibrary.MakeVector` (- (.x (`SplineComponent.GetLocationAtDistanceAlongSpline` _spline _returnvalue_2 "Local")) 15.0) (- (.y (`SplineComponent.GetLocationAtDistanceAlongSpline` _spline _returnvalue_2 "Local")) (`self.SegmentOffset_Y`)) (.z (`SplineComponent.GetLocationAtDistanceAlongSpline` _spline _returnvalue_2 "Local"))) (`KismetMathLibrary.ClampVectorSize` (`SplineComponent.GetTangentAtDistanceAlongSpline` _spline _returnvalue_2 "Local") 0.0 (`self.ChainSegmentLength`)) (`SplineComponent.GetLocationAtDistanceAlongSpline` _spline _returnvalue_3 "Local") (`KismetMathLibrary.ClampVectorSize` (`SplineComponent.GetTangentAtDistanceAlongSpline` _spline _returnvalue_3 "Local") 0.0 (`self.ChainSegmentLength`)) true)))