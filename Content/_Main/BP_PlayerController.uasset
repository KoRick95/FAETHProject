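; Player controller that owns the player's UI and joins the networked dungeon-build handshake.
; On possession it creates the HUD and passive skill grid client-side, finding the existing inventory widget after a short delay.
; Wrapper events forward resource orbs, boss bar, pickup, death, survey and menu toggles to Client events; menu opens log analytics, and Pause closes inventory first.
; Clients build the dungeon from a supplied seed, then notify the GameMode through the server.
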(event `self.ReceivePossess`
  (params (PossessedPawn :type "Pawn Object Reference"))
  (`self.Client_CreateHUD`))

(event `Client_CreateHUD`
  ;[1 1 1] Create HUD
  (if (`self.IsLocalPlayerController`)
    (`/Engine/EditorBlueprintResources/StandardMacros.IsValid` (`self.PlayerHUD`)
      (:`Is Valid`
        _)
      (:`Is Not Valid`
        (bind _returnvalue (`|CreateWidget` "/Game/_Main/UI/W_PlayerHUD.W_PlayerHUD_C" self))
        (bind _output_get (set `self.PlayerHUD` _returnvalue))))
    (`UserWidget.AddToViewport` _output_get 0)
    ;[1 1 1] Create Inventory HUD
    (`KismetSystemLibrary.Delay` 0.5)
    (bind _foundwidgets (`WidgetBlueprintLibrary.GetAllWidgetsOfClass` "/Game/_Main/Inventory/Widgets/W_InventoryHUD.W_InventoryHUD_C" false))
    (set `self.InventoryHUD` (`|GetArrayItem` _foundwidgets))
    ;[1 1 1] Create Passive Skill Grid
    (bind _returnvalue_2 (`|CreateWidget` "/Game/_Main/PassiveGrid/W_PassiveGrid.W_PassiveGrid_C"))
    (bind _output_get_2 (set `self.SkillGrid` _returnvalue_2))
    (`UserWidget.AddToViewport` _output_get_2 0)))

(event `/Game/_Main/Interfaces/INT_PlayerController.UpdateHealthUI`
  (params (HealthPercent :type "Float (single-precision)"))
  ;[1 1 1] Player Resources
  (`self.Client_UpdateHealthUI` HealthPercent))

(event `Client_UpdateHealthUI`
  (params (Health :type "Float (double-precision)"))
  ;[1 1 1] Player Resources
  (`/Game/_Main/UI/W_GlassOrb.SetPercentage` (`/Game/_Main/UI/W_PlayerHUD.GlassOrb_Health` (`self.PlayerHUD`)) Health))

(event `/Game/_Main/Interfaces/INT_PlayerController.UpdateManaUI`
  (params (ManaPercent :type "Float (single-precision)"))
  ;[1 1 1] Player Resources
  (`self.Client_UpdateManaUI` ManaPercent))

(event `Client_UpdateManaUI`
  (params (Mana :type "Float (double-precision)"))
  ;[1 1 1] Player Resources
  (`/Game/_Main/UI/W_GlassOrb.SetPercentage` (`/Game/_Main/UI/W_PlayerHUD.GlassOrb_Mana` (`self.PlayerHUD`)) Mana))

(event `/Game/_Main/Interfaces/INT_PlayerController.UpdateStaminaUI`
  (params (StaminaPercent :type "Float (single-precision)"))
  ;[1 1 1] Player Resources
  (`self.Client_UpdateStaminaUI` StaminaPercent))

(event `Client_UpdateStaminaUI`
  (params (Stamina :type "Float (double-precision)"))
  (bind _playerhud (`self.PlayerHUD`))
  ;[1 1 1] Player Resources
  (`/Engine/EditorBlueprintResources/StandardMacros.IsValid` _playerhud
    (:`Is Valid`
      (`/Game/_Main/UI/W_GlassOrb.SetPercentage` (`/Game/_Main/UI/W_PlayerHUD.GlassOrb_Stamina` _playerhud) Stamina))))

(event `/Game/_Main/Interfaces/INT_PlayerController.ToggleBossInfoOverlay`
  (params (Visibility :type "ESlateVisibility Enum" :default "Visible") (BossName :type Text))
  ;[1 1 1] Boss Bar
  (`self.Client_ToggleBossInfoOverlay` Visibility BossName))

(event `Client_ToggleBossInfoOverlay`
  (params (Visibility :type "ESlateVisibility Enum" :default "Visible") (BossName :type Text))
  ;[1 1 1] Boss Bar
  (`/Game/_Main/UI/W_PlayerHUD.ToggleBossInfoOverlay` (`self.PlayerHUD`) Visibility BossName))

(event `/Game/_Main/Interfaces/INT_PlayerController.UpdateBossHealthBar`
  (params (PercentHealth :type "Float (single-precision)"))
  ;[1 1 1] Boss Bar
  (`self.Client_UpdateBossHealthBar` PercentHealth))

(event `Client_UpdateBossHealthBar`
  (params (PercentHealth :type "Float (double-precision)"))
  ;[1 1 1] Boss Bar
  (`/Game/_Main/UI/W_PlayerHUD.UpdateBossHPBar` (`self.PlayerHUD`) PercentHealth))

(event `/Game/_Main/Interfaces/INT_PlayerController.DeathScreen`
  ;[1 1 1] Death Screen
  (`self.Client_CreateDeathScreen`))

(event `Client_CreateDeathScreen`
  ;[1 1 1] Death Screen
  (`WidgetLayoutLibrary.RemoveAllWidgets`)
  (bind _returnvalue (`|CreateWidget` "/Game/_Main/UI/W_DeathScreen.W_DeathScreen_C"))
  (`UserWidget.AddToViewport` _returnvalue 0))

(event `InputAction|Pause`
  (params (Key :type "Key Structure"))
  ;[1 1 1] Pause
  (:`Pressed`
    (if (not (`self.IsInventoryOpen`))
      (`self.PauseGame`)
      (else
        (`self.Client_ToggleInventory`)))))

(event `PauseGame`
  ;[1 1 1] Pause
  (if (`self.IsPauseMenuOpen`)
    (`GameplayStatics.SetGamePaused` false)
    (`/Game/_Main/UI/W_PauseMenu.ClosePauseMenu` (stale _returnvalue))
    (set `self.IsPauseMenuOpen` false)
    (`WidgetBlueprintLibrary.SetInputMode_GameOnly` self)
    (else
      (bind _returnvalue (`|CreateWidget` "/Game/_Main/UI/W_PauseMenu.W_PauseMenu_C" self))
      (`UserWidget.AddToViewport` _returnvalue 0)
      (`GameplayStatics.SetGamePaused` true)
      (set `self.IsPauseMenuOpen` true)
      (`WidgetBlueprintLibrary.SetInputMode_UIOnlyEx` self _returnvalue)))
  (set `self.bShowMouseCursor` (`self.IsPauseMenuOpen`)))

(event `/Game/_Main/Interfaces/INT_PlayerController.ToggleInventory`
  ;[1 1 1] Toggle Inventory
  (`self.Client_ToggleInventory`))

(event `Client_ToggleInventory`
  (bind _inventoryhud (`self.InventoryHUD`))
  ;[1 1 1] Toggle Inventory
  (if (not (`self.IsInventoryOpen`))
    (set `self.IsInventoryOpen` true)
    (`/Game/_Main/Inventory/Widgets/W_InventoryHUD.OpenInventory` _inventoryhud)
    (`GameAnalytics.AddDesignEventWithValue` "Open Inventory" 1.0)
    (else
      (`/Game/_Main/Inventory/Widgets/W_InventoryHUD.CloseInventory` _inventoryhud))))

(event `/Game/_Main/Interfaces/INT_PlayerController.TogglePassiveGrid`
  (`self.Client_ToggleSkillGrid`))

(event `Client_ToggleSkillGrid`
  (bind _skillgrid (`self.SkillGrid`))
  (if (not (`self.IsSkillGridOpen`))
    (set `self.IsSkillGridOpen` true)
    (`/Game/_Main/PassiveGrid/W_PassiveGrid.OpenPassiveGrid` _skillgrid)
    (`GameAnalytics.AddDesignEventWithValue` "Open Skill Grid" 1.0)
    (else
      (`/Game/_Main/PassiveGrid/W_PassiveGrid.ClosePassiveGrid` _skillgrid))))

(event `/Game/_Main/Interfaces/INT_PlayerController.ShowPickupName`
  (params (State :type Boolean) (Name :type Text))
  ;[1 1 1] Pickup Name
  (`self.Client_ShowPickupName` State Name))

(event `Client_ShowPickupName`
  (params (State :type Boolean) (Message :type Text))
  ;[1 1 1] Pickup Name
  (`/Game/_Main/UI/W_PlayerHUD.PlayerMessage` (`self.PlayerHUD`) State Message))

(event `/Game/_Main/Interfaces/INT_PlayerController.SurveyScreen`
  ;[1 1 1] Survey
  (`self.Client_CreateSurveyScreen`))

(event `Client_CreateSurveyScreen`
  ;[1 1 1] Survey
  (bind _returnvalue (`|CreateWidget` "/Game/_Main/UI/W_SurveyScreen.W_SurveyScreen_C"))
  (`UserWidget.AddToViewport` _returnvalue 0)
  (set `self.bShowMouseCursor` true))

(event `Client_BuildDungeon`
  (params (DungeonSeed :type Integer))
  (bind _dungeon (`/DungeonArchitect/Samples/DA_MultiplayerDemo/Blueprints/DA_MPV_Utils.FindDungeonActor`))
  (`/Engine/EditorBlueprintResources/StandardMacros.IsValid` _dungeon
    (:`Is Valid`
      (set `DungeonConfig.Seed` DungeonSeed (`Dungeon.Config` _dungeon))
      (add `Dungeon.OnDungeonBuildComplete` _dungeon (delegate `OnBuildComplete`))
      (`Dungeon.BuildDungeon` _dungeon))))

(event `OnBuildComplete`
  (params (Dungeon :type "Dungeon Object Reference") (bSuccess :type Boolean))
  (`self.Server_NotifyBuildComplete`))

(event `Server_NotifyBuildComplete`
  (bind _asbp_game_mode (cast `/Game/_Main/BP_GameMode` (`GameplayStatics.GetGameMode`)))
  (`/Game/_Main/BP_GameMode.F_NotifyPlayerReady` _asbp_game_mode))

(fn `ControllerRef`
  (returns (ControllerRef :type "/Game/_Main/BP_PlayerController Object Reference"))
  (return self))

(fn `UserConstructionScript`)