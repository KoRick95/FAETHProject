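; BP_CharacterBase is a base character Blueprint that provides a PushCharacter event for knockbacks.
; The event plays the pushed montage and applies a velocity-change impulse with ground friction zeroed, then restores friction with no delay.
; FSetCollisionToPawn brackets the push with Ignore and Block, but changes the capsule's WorldStatic response despite its name.
; The StunDuration input is unused.
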(event `PushCharacter`
  (params (ImpulseDirection :type "Vector Structure") (PushStrength :type "Float (double-precision)") (StunDuration :type "Float (double-precision)") (PushedAnimation :type "AnimMontage Object Reference"))
  (`self.F_SetCollisionToPawn` "ECR_Ignore")
  (`self.PlayAnimMontage` PushedAnimation)
  (set `self.DefaultGroundFriction` (`CharacterMovementComponent.GroundFriction` (`self.CharacterMovement`)))
  (set `CharacterMovementComponent.GroundFriction` 0.0 (`self.CharacterMovement`))
  (`CharacterMovementComponent.AddImpulse` (`self.CharacterMovement`) (* ImpulseDirection PushStrength) true)
  (set `CharacterMovementComponent.GroundFriction` (`self.DefaultGroundFriction`) (`self.CharacterMovement`))
  (`self.F_SetCollisionToPawn` "ECR_Block"))

(fn `F_SetCollisionToPawn`
  (params (NewResponse :type "ECollisionResponse Enum" :default "ECR_Ignore"))
  (`PrimitiveComponent.SetCollisionResponseToChannel` (`self.CapsuleComponent`) "ECC_WorldStatic" NewResponse))

(fn `UserConstructionScript`)