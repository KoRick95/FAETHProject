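; Base gameplay ability Blueprint providing shared helpers for player and enemy abilities, with no activation or end logic of its own.
; Helpers resolve player or enemy character and controller references through interface-style Ref messages.
; A resource check negates the ability's cost and tests whether the player's current Health, Mana or Stamina attribute strictly exceeds it.
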(fn `F_GetEnemyCharacterAndController`
  (returns (EnemyRef :type "/Game/_Main/AI/BP_EnemyBase Object Reference") (AICRef :type "AIController Object Reference"))
  (bind _enemyref (message `/Game/_Main/Interfaces/INT_EnemyAI.EnemyRef` (`self.GetOwningActorFromActorInfo`)))
  (bind _aicref (message `/Game/_Main/Interfaces/INT_AIController.AICRef` (`AIBlueprintHelperLibrary.GetAIController` null)))
  (return _enemyref _aicref))

(fn `F_GetPlayerCharacterAndController`
  (returns (PlayerRef :type "/Game/_Main/Characters/BP_PlayerCharacter Object Reference") (ControllerRef :type "/Game/_Main/BP_PlayerController Object Reference"))
  (bind _playerref (message `/Game/_Main/Interfaces/INT_PlayerCharacter.PlayerRef` (`self.GetOwningActorFromActorInfo`)))
  (bind _controllerref (message `/Game/_Main/Interfaces/INT_PlayerController.ControllerRef` (`Pawn.GetController` _playerref)))
  (return _playerref _controllerref))

(fn `F_IsResourceStillAvailable`
  (params (Resource :type String))
  (returns (Can :type Boolean))
  (locals (Cost :type "Float (double-precision)" :default 0.0))
  (bind _returnvalue (`self.GetAbilityCost` Resource))
  (set `local.Cost` (* _returnvalue -1.0))
  (switch `string` Resource
    (:`Health`
      (bind _playerref (`self.F_GetPlayerCharacterAndController`))
      (bind (_health_basevalue _health_currentvalue) (break `GameplayAttributeData` (`CharacterAttributeSet.Health` (`BaseCharacter.CharacterAttributeSet` _playerref))))
      (return (> _health_currentvalue (`local.Cost`))))
    (:`Mana`
      (bind _playerref_2 (`self.F_GetPlayerCharacterAndController`))
      (bind (_mana_basevalue _mana_currentvalue) (break `GameplayAttributeData` (`CharacterAttributeSet.Mana` (`BaseCharacter.CharacterAttributeSet` _playerref_2))))
      (return (> _mana_currentvalue (`local.Cost`))))
    (:`Stamina`
      (bind _playerref_3 (`self.F_GetPlayerCharacterAndController`))
      (bind (_stamina_basevalue _stamina_currentvalue) (break `GameplayAttributeData` (`CharacterAttributeSet.Stamina` (`BaseCharacter.CharacterAttributeSet` _playerref_3))))
      (return (> _stamina_currentvalue (`local.Cost`))))))