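; Player inventory component that creates the inventory HUD, handles equipping and unequipping gear, and spawns dropped loot as pickups.
; Equipped items live in a map keyed by equipment type, with swaps updating equipment slot UI and the main-hand mesh.
; Stat updates reset player attributes, then add item stats, completed-set bonuses from data tables and slot connection bonuses from the equipment widget.
; Server and multicast events wrap equipping, stat changes and loot drops.
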(event `InitialiseInventory`)

(event `self.ReceiveBeginPlay`
  (`KismetSystemLibrary.Delay` 0.2)
  (`self.Client_CreateInventory`))

(event `Client_CreateInventory`
  (bind _playerref (message `/Game/_Main/Interfaces/INT_PlayerCharacter.PlayerRef` (`GameplayStatics.GetPlayerCharacter` 0)))
  (set `self.Player Ref` _playerref)
  (bind _returnvalue (`|CreateWidget` "/Game/_Main/Inventory/Widgets/W_InventoryHUD.W_InventoryHUD_C"))
  (bind _output_get (set `self.MainHUD` _returnvalue))
  (`UserWidget.AddToViewport` _output_get 0)
  (`UserWidget.AddToViewport` _returnvalue 0)
  (`/Game/_Main/Inventory/Libraries/BPFL_Inventory.InitialiseInventory` 16 (make `Anchors` (-0.6 0.3) (1.35 0.6)))
  (`Widget.SetVisibility` _returnvalue "Collapsed")
  (bind _foundwidgets (`WidgetBlueprintLibrary.GetAllWidgetsOfClass` "/Game/_Main/Inventory/Widgets/W_EquipmentInventory.W_EquipmentInventory_C" false))
  (set `self.EquipmentInventoryHUD` (`|GetArrayItem` _foundwidgets))
  (`self.UpdateStats`))

(event `Server_EquipItem`
  (params (ItemData :type "/Game/_Main/Inventory/Structs/ST_ItemData Structure") (Slot :type "/Game/_Main/Inventory/Widgets/W_Slot Object Reference") (ItemWasSwapped :type Boolean) (PreviousItemData :type "/Game/_Main/Inventory/Structs/ST_ItemData Structure") (DontRemovePreviousItem :type Boolean))
  (`self.EquipItem` ItemData Slot ItemWasSwapped PreviousItemData DontRemovePreviousItem))

(event `Server_UnequipItem`
  (params (EquipmentType :type "/Game/_Main/Inventory/Enums/E_EquipmentTypes Enum" :default "NewEnumerator0"))
  (`self.UnequipItem` EquipmentType))

(event `Server_AddStats`
  (params (Stats :type "/Game/_Main/Inventory/Structs/ST_Stats Structure"))
  (`self.AddStats` Stats))

(event `Multi_DropLoot`
  (params (Item :type "DataTableRowHandle Structure") (SpawnTransform :type "Transform Structure"))
  (`self.DropLoot` Item SpawnTransform))

(fn `AddStats`
  (params (Stats :type "/Game/_Main/Inventory/Structs/ST_Stats Structure"))
  (bind (_health _mana _stamina _strength) (break `/Game/_Main/Inventory/Structs/ST_Stats` Stats))
  (bind _player_ref (`self.Player Ref`))
  (bind _player_ref_2 (`self.Player Ref`))
  (bind _player_ref_3 (`self.Player Ref`))
  (bind _strength_basevalue (break `GameplayAttributeData` (`CharacterAttributeSet.Strength` (`BaseCharacter.CharacterAttributeSet` (`self.Player Ref`)))))
  (bind _maxstamina_basevalue (break `GameplayAttributeData` (`CharacterAttributeSet.MaxStamina` (`BaseCharacter.CharacterAttributeSet` _player_ref_3))))
  (bind _maxmana_basevalue (break `GameplayAttributeData` (`CharacterAttributeSet.MaxMana` (`BaseCharacter.CharacterAttributeSet` _player_ref_2))))
  (bind _maxhealth_basevalue (break `GameplayAttributeData` (`CharacterAttributeSet.MaxHealth` (`BaseCharacter.CharacterAttributeSet` _player_ref))))
  (`|ExecutionSequence`
    (:`then_0`
      ;[1 1 1] Health
      (`BaseCharacter.SetMaxHealth` _player_ref (+ _maxhealth_basevalue _health)))
    (:`then_1`
      ;[1 1 1] Mana
      (`BaseCharacter.SetMaxMana` _player_ref_2 (+ _maxmana_basevalue _mana)))
    (:`then_2`
      ;[1 1 1] Stamina
      (`BaseCharacter.SetMaxStamina` _player_ref_3 (+ _maxstamina_basevalue _stamina)))
    (:`then_3`
      ;[1 1 1] Strength
      (`BaseCharacter.SetStrength` (`self.Player Ref`) (+ _strength_basevalue _strength)))))

(fn `AddToStat`
  (params (StatToChange :type "Float (double-precision) (by ref)") (StatToAdd :type "Float (double-precision)"))
  (returns (StatValue :type "Float (double-precision)"))
  (bind _returnvalue (+ StatToChange StatToAdd))
  (`|VariableSetRef` StatToChange _returnvalue)
  (return _returnvalue))

(fn `CalculateBaseStats`
  (bind _values (`BlueprintMapLibrary.Map_Values` (`self.EquippedItems`)))
  (for _array_element _values
    (`self.Server_AddStats` (`.Stats_9_B57B10BD44690EC10AC560BA04519CE5` (break `/Game/_Main/Inventory/Structs/ST_EquipmentData` (`.EquipmentData_26_EC58DB734B5EA2A0A265068585053002` (break `/Game/_Main/Inventory/Structs/ST_ItemData` _array_element)))))))

(fn `CalculateConnectionStats`
  (bind _connectionstats (`/Game/_Main/Inventory/Widgets/W_EquipmentInventory.CheckConnections` (`self.EquipmentInventoryHUD`)))
  (for _array_element _connectionstats
    (`self.Server_AddStats` _array_element)))

(fn `CalculateSetStats`
  (locals (PotentialSets :type "Array of /Game/_Main/Inventory/Structs/ST_EquipmentSet Structure") (SetIsValid :type Boolean))
  (bind _potentialsets (`local.PotentialSets`))
  ;[1 1 1] Find all potential sets in inventory
  (bind _values (`BlueprintMapLibrary.Map_Values` (`self.EquippedItems`)))
  (for _array_element _values
    (bind _returnvalue (`|GetDataTableRow` "/Game/_Main/Inventory/DataTables/DT_EquipmentSets.DT_EquipmentSets" (`.RowName` (break `DataTableRowHandle` (`.EquipmentSet_10_9E654AF3416B43D16A3EF6B1E7330101` (break `/Game/_Main/Inventory/Structs/ST_EquipmentData` (`.EquipmentData_26_EC58DB734B5EA2A0A265068585053002` (break `/Game/_Main/Inventory/Structs/ST_ItemData` _array_element)))))))
      (:`then`
        (if (not (`KismetArrayLibrary.Array_Contains` _potentialsets _returnvalue))
          (`KismetArrayLibrary.Array_Add` _potentialsets _returnvalue)))))
  (`BlueprintMapLibrary.Map_Clear` (`/Game/_Main/Inventory/Widgets/W_EquipmentInventory.ActiveSets` (`self.EquipmentInventoryHUD`)))
  (for _array_element_2 (`local.PotentialSets`)
    (set `local.SetIsValid` false)
    (bind (_name _equipmentpieces _stats) (break `/Game/_Main/Inventory/Structs/ST_EquipmentSet` _array_element_2))
    ;[1 1 1] Check if all the pieces in the set are equipped
    (for _array_element_3 _equipmentpieces
      (bind _returnvalue_2 (`|GetDataTableRow` "/Game/_Main/Inventory/DataTables/DT_Items.DT_Items" (`.RowName` (break `DataTableRowHandle` _array_element_3)))
        (:`then`
          (bind (_name_2 _types _description _icon _mesh _rarity _quantity _stackable _equipmentdata) (break `/Game/_Main/Inventory/Structs/ST_ItemData` _returnvalue_2))
          (if (== (`.Name_18_D0186B6F4758389A94E4EDB0A5287F40` (break `/Game/_Main/Inventory/Structs/ST_ItemData` (`BlueprintMapLibrary.Map_Find` (`self.EquippedItems`) (`.EquipmentType_8_6108977F4F05136470B412A731B49EB5` (break `/Game/_Main/Inventory/Structs/ST_EquipmentData` _equipmentdata))))) _name_2)
            (set `local.SetIsValid` true)
            (else
              (set `local.SetIsValid` false)
              (break))))
        (:`RowNotFound`
          (set `local.SetIsValid` false)
          (break))))
    ;[1 1 1] If all required items are equipped, apply set stats
    (if (`local.SetIsValid`)
      (`self.Server_AddStats` _stats)
      (`BlueprintMapLibrary.Map_Add` (`/Game/_Main/Inventory/Widgets/W_EquipmentInventory.ActiveSets` (`self.EquipmentInventoryHUD`)) (`KismetStringLibrary.Conv_NameToString` _name) _stats)))
  (`/Game/_Main/Inventory/Widgets/W_EquipmentInventory.GetActiveSets` (`self.EquipmentInventoryHUD`)))

(fn `DropLoot`
  (params (Item :type "DataTableRowHandle Structure") (SpawnTransform :type "Transform Structure"))
  (bind _returnvalue (`|SpawnActorFromClass` "/Game/_Main/Interactables/BP_BasePickup.BP_BasePickup_C" SpawnTransform "Undefined" "OverrideRootScale" null null))
  (set `/Game/_Main/Interactables/BP_BasePickup.Item` Item _returnvalue)
  (`/Game/_Main/Interactables/BP_BasePickup.UpdateInfo` _returnvalue))

(fn `EquipItem`
  (params (ItemData :type "/Game/_Main/Inventory/Structs/ST_ItemData Structure") (Slot :type "/Game/_Main/Inventory/Widgets/W_Slot Object Reference") (ItemWasSwapped :type Boolean) (PreviousItemData :type "/Game/_Main/Inventory/Structs/ST_ItemData Structure") (DontRemovePreviousItem :type Boolean))
  (locals (ExistingItem :type "/Game/_Main/Inventory/Structs/ST_ItemData Structure") (ItemTypeToAdd :type "/Game/_Main/Inventory/Enums/E_EquipmentTypes Enum") (ItemToAdd :type "/Game/_Main/Inventory/Structs/ST_ItemData Structure") (UsedSlot :type "/Game/_Main/Inventory/Widgets/W_Slot Object Reference"))
  (bind _itemtypetoadd (`local.ItemTypeToAdd`))
  (bind _existingitem (`local.ExistingItem`))
  (bind _equippeditems (`self.EquippedItems`))
  (bind _existingitem_name (break `/Game/_Main/Inventory/Structs/ST_ItemData` (`local.ExistingItem`)))
  (bind (_name _types _description _icon _mesh _rarity _quantity _stackable _equipmentdata) (break `/Game/_Main/Inventory/Structs/ST_ItemData` (`local.ItemToAdd`)))
  (bind _equipmenttype (break `/Game/_Main/Inventory/Structs/ST_EquipmentData` (`.EquipmentData_26_EC58DB734B5EA2A0A265068585053002` (break `/Game/_Main/Inventory/Structs/ST_ItemData` PreviousItemData))))
  (set `local.UsedSlot` Slot)
  (bind _output_get (set `local.ItemToAdd` ItemData))
  (bind _output_get_2 (set `local.ItemTypeToAdd` (`.EquipmentType_8_6108977F4F05136470B412A731B49EB5` (break `/Game/_Main/Inventory/Structs/ST_EquipmentData` (`.EquipmentData_26_EC58DB734B5EA2A0A265068585053002` (break `/Game/_Main/Inventory/Structs/ST_ItemData` _output_get))))))
  (bind (_value _returnvalue) (`BlueprintMapLibrary.Map_Find` (`self.EquippedItems`) _output_get_2))
  ;[1 1 1] Check if item to add is already equipped
  (set `local.ExistingItem` _value)
  (if _returnvalue
    (if ItemWasSwapped
      ;[1 1 1] If equipment type is already equipped, remove currently equipped item and place it in inventory
      (`BlueprintMapLibrary.Map_Remove` (`self.EquippedItems`) (`.EquipmentType_8_6108977F4F05136470B412A731B49EB5` (break `/Game/_Main/Inventory/Structs/ST_EquipmentData` (`.EquipmentData_26_EC58DB734B5EA2A0A265068585053002` (break `/Game/_Main/Inventory/Structs/ST_ItemData` _existingitem)))) :!label _label)
      (`BlueprintMapLibrary.Map_Add` (`self.EquippedItems`) (`local.ItemTypeToAdd`) (`local.ItemToAdd`))
      ;[1 1 1] Clear previous existing item UI
      (bind _slots (`/Game/_Main/Inventory/Widgets/W_EquipmentInventory.FindSlotsWith` (`self.EquipmentInventoryHUD`) (`local.ExistingItem`)))
      (for _array_element _slots
        (if (!= (`/Game/_Main/Inventory/Widgets/W_Slot.Name` _array_element) (`/Game/_Main/Inventory/Widgets/W_Slot.Name` (`local.UsedSlot`)))
          (set `/Game/_Main/Inventory/Widgets/W_Slot.Information` (struct) _array_element)
          (`/Game/_Main/Inventory/Widgets/W_Slot.UpdateUI` _array_element)))
      ;[1 1 1] Remove previous item from map and update stats
      (if DontRemovePreviousItem :!label _label_2
        _
        (elif (`.ReturnValue` (`BlueprintMapLibrary.Map_Find` _equippeditems _equipmenttype))
          (`BlueprintMapLibrary.Map_Remove` _equippeditems _equipmenttype)))
      (`self.UpdateStats`)
      ;[1 1 1] If Previously Equipped Nothing
      (if (== _existingitem_name "None")
        ;[1 1 1] If a Main Hand Item Equipped, Change Player's Main Hand SM to the SM in the DT
        (if (`|EnumEquality` (`.EquipmentType_8_6108977F4F05136470B412A731B49EB5` (break `/Game/_Main/Inventory/Structs/ST_EquipmentData` _equipmentdata)) "NewEnumerator6") :!label _label_3
          (`/Game/_Main/Characters/BP_PlayerCharacter.F_SetMainHandMesh` (`self.Player Ref`) _mesh))
        (else
          ;[1 1 1] If Item to Add is the Same Type as Already Equipped
          (if (and (`|EnumEquality` (break `/Game/_Main/Inventory/Structs/ST_EquipmentData` (`.EquipmentData_26_EC58DB734B5EA2A0A265068585053002` (break `/Game/_Main/Inventory/Structs/ST_ItemData` (`local.ExistingItem`)))) _itemtypetoadd) (`|EnumEquality` _itemtypetoadd "NewEnumerator6"))
            (`/Game/_Main/Characters/BP_PlayerCharacter.F_SetMainHandMesh` (`self.Player Ref`) null)
            (goto _label_3))))
      (else
        (bind _successfullyadded (`/Game/_Main/Inventory/Libraries/BPFL_Inventory.AddItem` _existingitem))
        (if _successfullyadded
          (goto _label))))
    (else
      ;[1 1 1] Equip item
      (`BlueprintMapLibrary.Map_Add` (`self.EquippedItems`) (`local.ItemTypeToAdd`) (`local.ItemToAdd`))
      (goto _label_2))))

(fn `UnequipItem`
  (params (EquipmentType :type "/Game/_Main/Inventory/Enums/E_EquipmentTypes Enum" :default "NewEnumerator0"))
  (returns (Removed :type Boolean))
  (bind _returnvalue (`BlueprintMapLibrary.Map_Remove` (`self.EquippedItems`) EquipmentType))
  (if _returnvalue
    (if (not (`.ReturnValue` (`BlueprintMapLibrary.Map_Find` (`self.EquippedItems`) "NewEnumerator6")))
      (`/Game/_Main/Characters/BP_PlayerCharacter.F_SetMainHandMesh` (`self.Player Ref`) null)
      (`self.UpdateStats`)
      (return true))
    (else
      (return false))))

(fn `UpdateStats`
  (bind _player_ref (`self.Player Ref`))
  (bind _player_ref_2 (`self.Player Ref`))
  (bind _player_ref_3 (`self.Player Ref`))
  (bind _player_ref_4 (`self.Player Ref`))
  (bind _player_ref_5 (`self.Player Ref`))
  ;[1 1 1] Reset stats
  (`BaseCharacter.SetMaxHealth` _player_ref_2 (`/Game/_Main/Characters/BP_PlayerCharacter.StartHealth` _player_ref_2))
  (`BaseCharacter.SetMaxMana` _player_ref_3 (`/Game/_Main/Characters/BP_PlayerCharacter.StartMana` _player_ref_3))
  (`BaseCharacter.SetMaxStamina` _player_ref_4 (`/Game/_Main/Characters/BP_PlayerCharacter.StartStamina` _player_ref_4))
  (`BaseCharacter.SetStrength` _player_ref_5 (`/Game/_Main/Characters/BP_PlayerCharacter.PassiveStrength` _player_ref_5))
  (`BaseCharacter.SetStagger` _player_ref (`/Game/_Main/Characters/BP_PlayerCharacter.StartStagger` _player_ref))
  ;[1 1 1] Calculate all stats together
  (`self.CalculateBaseStats`)
  (`self.CalculateSetStats`)
  (`self.CalculateConnectionStats`))