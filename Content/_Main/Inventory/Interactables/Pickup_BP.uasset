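; Interactable item pickup that the player adds to the inventory by pressing E.
; On BeginPlay it looks up its data table row to set the mesh and the "[E]" name text on its nameplate widget.
; Overlap with a ThirdPersonCharacter shows the nameplate and enables input on the actor itself, and leaving reverses both.
; E passes the item info and quantity to AddItem, destroying the actor only if that succeeds.
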(event `self.ReceiveBeginPlay`
  (bind (_datatable _rowname) (break `DataTableRowHandle` (`self.Item`)))
  ;[1 1 1] Get Item Information
  (bind _returnvalue (`|GetDataTableRow` _datatable _rowname)
    (:`then`
      (set `self.Information` _returnvalue)
      (`StaticMeshComponent.SetStaticMesh` (`self.Model`) (`.Model_20_6166920D457D39C9C69D1F9368E6DBC1` (break `/Game/Inventory/Structs/ItemData` (`self.Information`))))
      ;[1 1 1] Update Nameplate
      (bind _aspickup_nameplate_wg (cast `/Game/Inventory/Interactables/PickupNameplate_WG` (`WidgetComponent.GetUserWidgetObject` (`self.Nameplate`))))
      (`TextBlock.SetText` (`/Game/Inventory/Interactables/PickupNameplate_WG.NameText` _aspickup_nameplate_wg) (`KismetTextLibrary.Conv_StringToText` (`KismetStringLibrary.Concat_StrStr` "[E]" (`KismetStringLibrary.Conv_NameToString` (`.Name_16_D9613DD04E66486E650D3EB0CBC39E25` (break `/Game/Inventory/Structs/ItemData` (`self.Information`))))))))))

(event `self.InteractionCollider.OnComponentBeginOverlap`
  (params (OverlappedComponent :type "PrimitiveComponent Object Reference") (OtherActor :type "Actor Object Reference") (OtherComp :type "PrimitiveComponent Object Reference") (OtherBodyIndex :type Integer) (bFromSweep :type Boolean) (SweepResult :type "HitResult Structure (by ref)"))
  ;[1 1 1] On player enter
  (if (`KismetMathLibrary.ClassIsChildOf` (`GameplayStatics.GetObjectClass` OtherActor) "/Game/ThirdPersonBP/Blueprints/ThirdPersonCharacter.ThirdPersonCharacter_C")
    (`SceneComponent.SetVisibility` (`self.Nameplate`) true false)
    (`self.EnableInput` (`GameplayStatics.GetPlayerController` 0))))

(event `self.InteractionCollider.OnComponentEndOverlap`
  (params (OverlappedComponent :type "PrimitiveComponent Object Reference") (OtherActor :type "Actor Object Reference") (OtherComp :type "PrimitiveComponent Object Reference") (OtherBodyIndex :type Integer))
  ;[1 1 1] On player exit
  (if (`KismetMathLibrary.ClassIsChildOf` (`GameplayStatics.GetObjectClass` OtherActor) "/Game/ThirdPersonBP/Blueprints/ThirdPersonCharacter.ThirdPersonCharacter_C")
    (`SceneComponent.SetVisibility` (`self.Nameplate`) false false)
    (`self.DisableInput` (`GameplayStatics.GetPlayerController` 0))))

(event `Key|E`
  (params (Key :type "Key Structure"))
  (bind _information (`self.Information`))
  ;[1 1 1] Add to inventory and destroy
  (:`Pressed`
    (bind _successfullyadded (`/Game/Inventory/Libraries/Inventory_BPFL.AddItem` _information (`.Quantity_22_D0F4FA134F4CCF70B78167A95F829F3E` (break `/Game/Inventory/Structs/ItemData` _information))))
    (if _successfullyadded
      (`self.K2_DestroyActor`))))

(fn `UserConstructionScript`)