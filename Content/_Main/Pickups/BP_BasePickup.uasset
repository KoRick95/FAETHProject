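; Base pickup actor with a static mesh and a sphere component.
; It turns on physics simulation for the mesh at BeginPlay.
; A DisablePhysics event stops the simulation and turns off collision on both the mesh and the sphere.
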(event `self.ReceiveBeginPlay`
  (`parent.ReceiveBeginPlay`)
  (`PrimitiveComponent.SetSimulatePhysics` (`self.StaticMesh`) true))

(event `/Game/_Main/Interfaces/INT_Pickups.DisablePhysics`
  (`PrimitiveComponent.SetSimulatePhysics` (`self.StaticMesh`) false)
  (`PrimitiveComponent.SetCollisionEnabled` (`self.StaticMesh`) "NoCollision")
  (`PrimitiveComponent.SetCollisionEnabled` (`self.Sphere`) "NoCollision"))

(fn `UserConstructionScript`
  (`parent.UserConstructionScript`))