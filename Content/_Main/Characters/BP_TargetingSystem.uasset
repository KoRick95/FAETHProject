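; BP_TargetingSystem gives its owning player pawn a toggleable lock-on to the nearest living enemy.
; A sphere overlap collects BP_EnemyBase actors within the scan radius, and the closest becomes the locked target.
; Interface messages pass the target to the pawn and toggle the enemy's target widget.
; A looping timer releases the lock when the target moves beyond the scan radius.
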(event `Initialise`
  (bind _output_get (set `self.PlayerPawn` (cast `Pawn` (`self.GetOwner`) :!pure true)))
  (bind _controllerref (message `/Game/_Main/Interfaces/INT_PlayerController.ControllerRef` (`Pawn.GetController` _output_get)))
  (set `self.PlayerController` _controllerref))

(event `LockOnTarget`
  (if (not (`self.IsTargeting`))
    (`self.FindTargets`)
    (else
      (`self.ToggleCameraLock` false))))

(event `FindTargets`
  ;[1 1 1] Scan for All Enemy BP Targets
  (bind _outactors (`KismetSystemLibrary.SphereOverlapActors` (`Actor.K2_GetActorLocation` (`self.PlayerPawn`)) (`self.ScanRadius`) (`|MakeArray` "ObjectTypeQuery3" :!type "EObjectTypeQuery Enum") "/Game/_Main/AI/BP_EnemyBase.BP_EnemyBase_C"))
  (for _array_element _outactors
    (bind _isdead (message `/Game/_Main/Interfaces/INT_EnemyAI.IsAIDead` _array_element))
    (if (not _isdead)
      (`KismetArrayLibrary.Array_AddUnique` (`self.PotentialTargets`) _array_element)))
  ;;[1 1 1] Set the Closest Target as the Locked Target
  (for _array_element_2 (`self.PotentialTargets`)
    (bind _returnvalue (`Actor.GetDistanceTo` (`self.PlayerPawn`) _array_element_2))
    (if (<= _returnvalue (`self.ClosestDistance`))
      (set `self.ClosestDistance` _returnvalue)
      (set `self.LockedTarget` _array_element_2)))
  ;[1 1 1] Reset the Closest Distance for Future Targeting, Clear Potential Targets and Start Targeting
  (set `self.ClosestDistance` (`self.ScanRadius`))
  (`KismetArrayLibrary.Array_Clear` (`self.PotentialTargets`))
  (`self.LockedTarget`
    (:`then`
      (set `self.IsTargeting` true)
      (`self.ToggleCameraLock` true)
      (bind _returnvalue_2 (`KismetSystemLibrary.K2_SetTimerDelegate` (delegate `CheckTargetDistance`) 0.25 true))
      (set `self.LockHandle` _returnvalue_2))
    (:`else`)))

(event `ToggleCameraLock`
  (params (State :type Boolean))
  (if State
    (set `self.IsTargeting` true)
    (message `/Game/_Main/Interfaces/INT_PlayerCharacter.SetTarget` (`self.PlayerPawn`) true (`self.LockedTarget`))
    (message `/Game/_Main/Interfaces/INT_EnemyAI.ToggleTargetWidget` (`self.LockedTarget`) true (`self.GetOwner`))
    (else
      (set `self.IsTargeting` false)
      (message `/Game/_Main/Interfaces/INT_PlayerCharacter.SetTarget` (`self.PlayerPawn`) false null)
      (message `/Game/_Main/Interfaces/INT_EnemyAI.ToggleTargetWidget` (`self.LockedTarget`) false (`self.GetOwner`))
      (set `self.LockedTarget` null))))

(event `CheckTargetDistance`
  ;[1 1 1] If Distance > Scan Radius, Stop Targeting
  (`self.LockedTarget`
    (:`then`
      (if (> (`Actor.GetDistanceTo` (`self.LockedTarget`) (`self.PlayerPawn`)) (`self.ScanRadius`))
        (`self.ToggleCameraLock` false)
        (`KismetSystemLibrary.K2_ClearAndInvalidateTimerHandle` (`self.LockHandle`))))
    (:`else`)))