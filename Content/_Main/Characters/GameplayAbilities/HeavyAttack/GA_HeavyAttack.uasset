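; Gameplay Ability for the player's heavy melee attack, playing a combo montage and applying damage on hits.
; On activation it commits, gets the montage from the player's FDetermineHeavyCombo and plays it.
; While waiting on Skill.melee.dealDamage events, it applies GE_HeavyAttack_Damage to each event target at the player's MeleeComboDamageLevel.
; The ability ends when the montage completes, blends out, is interrupted or is cancelled.
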(event `self.K2_ActivateAbility`
  (`parent.K2_ActivateAbility`)
  (`self.K2_CommitAbility`)
  (bind _playerref (message `/Game/_Main/Interfaces/INT_PlayerCharacter.PlayerRef` (`self.GetOwningActorFromActorInfo`)))
  (bind _montagetoplay (`/Game/_Main/Characters/BP_PlayerCharacter.F_DetermineHeavyCombo` _playerref))
  (`AbilityTask_PlayMontageAndWait.CreatePlayMontageAndWaitProxy` "None" _montagetoplay
    (:`then`
      (bind (_asynctaskproxy _payload) (`AbilityTask_WaitGameplayEvent.WaitGameplayEvent` (struct :`TagName` "skill.melee.dealDamage") null)
        (:`EventReceived`
          (bind (_eventtag _instigator _target) (break `GameplayEventData` _payload))
          (`self.BP_ApplyGameplayEffectToTarget` (`AbilitySystemBlueprintLibrary.AbilityTargetDataFromActor` _target) "/Game/_Main/Characters/GameplayAbilities/HeavyAttack/GE_HeavyAttack_Damage.GE_HeavyAttack_Damage_C" (`/Game/_Main/Characters/BP_PlayerCharacter.MeleeComboDamageLevel` _playerref))
          (message `/Game/_Main/Interfaces/INT_EnemyAI.EnemyRef` _target))))
    (:`OnCompleted`
      (`self.K2_EndAbility` :!label _label))
    (:`OnBlendOut`
      (goto _label))
    (:`OnInterrupted`
      (goto _label))
    (:`OnCancelled`
      (goto _label))))