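; Gameplay ability that makes the player sprint while Stamina lasts.
; After committing, it listens for Skill.sprint gameplay events and checks Stamina whenever one arrives.
; With Stamina available, it applies the sprint cost effect and sets max walk speed to SprintSpeed.
; Otherwise it removes drain effects by asset tag, applies stamina regen, restores JogSpeed and ends the ability.
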(event `self.K2_ActivateAbility`
  (`parent.K2_ActivateAbility`)
  (`self.K2_CommitAbility`)
  (`AbilityTask_WaitGameplayEvent.WaitGameplayEvent` (struct :`TagName` "skill.sprint") null
    (:`EventReceived`
      (bind _can (`self.F_IsResourceStillAvailable` "Stamina"))
      (if _can
        (`self.BP_ApplyGameplayEffectToOwner` "/Game/_Main/Characters/GameplayAbilities/Sprint/GE_Sprint_Cost.GE_Sprint_Cost_C")
        (bind _playerref (`self.F_GetPlayerCharacterAndController`))
        (set `CharacterMovementComponent.MaxWalkSpeed` (`self.SprintSpeed`) (`Character.CharacterMovement` _playerref))
        (else
          (`self.BP_RemoveGameplayEffectFromOwnerWithAssetTags` (struct :`GameplayTags` (struct :`(TagName` "skill.sprint.drainCost"))))
          (`self.BP_ApplyGameplayEffectToOwner` "/Game/_Main/Characters/GameplayAbilities/GeneralGameplayEffects/GE_StaminaRegen.GE_StaminaRegen_C")
          (bind _playerref_2 (`self.F_GetPlayerCharacterAndController`))
          (set `CharacterMovementComponent.MaxWalkSpeed` (`self.JogSpeed`) (`Character.CharacterMovement` _playerref_2))
          (`self.K2_EndAbility`))))))