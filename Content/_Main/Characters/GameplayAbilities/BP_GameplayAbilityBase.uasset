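; Base Gameplay Ability Blueprint that provides shared helpers for fetching player and enemy references.
; One helper gets the player character from the ability's owning actor and its controller from that character.
; The other gets the enemy from the owning actor and its AI controller through GetAIController.
; References resolve through interface messages rather than casts, and the activate and end events are unimplemented.
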(fn `F_GetEnemyCharacterAndController`
  (returns (EnemyRef :type "/Game/_Main/AI/BP_EnemyBase Object Reference") (AICRef :type "AIController Object Reference"))
  (bind _enemyref (message `/Game/_Main/Interfaces/INT_EnemyAI.EnemyRef` (`self.GetOwningActorFromActorInfo`)))
  (bind _aicref (message `/Game/_Main/Interfaces/INT_AIController.AICRef` (`AIBlueprintHelperLibrary.GetAIController` null)))
  (return _enemyref _aicref))

(fn `F_GetPlayerCharacterAndController`
  (returns (PlayerRef :type "/Game/_Main/Characters/BP_PlayerCharacter Object Reference") (ControllerRef :type "/Game/_Main/BP_PlayerController Object Reference"))
  (bind _playerref (message `/Game/_Main/Interfaces/INT_PlayerCharacter.PlayerRef` (`self.GetOwningActorFromActorInfo`)))
  (bind _controllerref (message `/Game/_Main/Interfaces/INT_PlayerController.ControllerRef` (`Pawn.GetController` _playerref)))
  (return _playerref _controllerref))