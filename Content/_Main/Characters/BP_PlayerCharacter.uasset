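; Player character for a networked melee action RPG, handling movement, sprint, block, dodge, combos, pickups and death.
; Combat runs through GAS: input activates melee, heavy, dodge and potion abilities, while authority sphere overlaps send damage events.
; Server events and OnRep functions push replicated states to the AnimInstance, and resource changes reach the UI through controller messages.
; NextAction enables animation cancelling by blending out montages and briefly ignoring root motion.
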(event `Key|R`
  (params (Key :type "Key Structure"))
  (:`Pressed`
    (bind _returnvalue (`|GetDataTableRow` "/Game/_Main/Inventory/DataTables/DT_Items.DT_Items" "AmuletOfPower")
      (:`then`
        (`/Game/_Main/Inventory/Libraries/BPFL_Inventory.AddItem` _returnvalue)))))

(event `self.ReceivePossessed`
  (params (NewController :type "Controller Object Reference"))
  (`self.UpdateMovement` true))

(event `self.ReceiveBeginPlay`
  (`AnalyticsBlueprintLibrary.StartSession`)
  (`KismetSystemLibrary.Delay` 0.25)
  (`self.GainAbility` "/Game/_Main/Characters/GameplayAbilities/Potion/GA_Potion.GA_Potion_C")
  (`self.GainAbility` "/Game/_Main/Characters/GameplayAbilities/Melee/GA_Melee.GA_Melee_C")
  (`self.GainAbility` "/Game/_Main/Characters/GameplayAbilities/Dodge/GA_Dodge.GA_Dodge_C")
  (`self.GainAbility` "/Game/_Main/Characters/GameplayAbilities/HeavyAttack/GA_HeavyAttack.GA_HeavyAttack_C")
  (`AbilitySystemComponent.BP_ApplyGameplayEffectToSelf` :`self` (`self.AbilitySystemComponent`) :`GameplayEffectClass` "/Game/_Main/Characters/GameplayAbilities/GeneralGameplayEffects/GE_StaminaRegen.GE_StaminaRegen_C"))

(event `InputAxis|Turn`
  (params (AxisValue :type "Float (single-precision)"))
  ;[1 1 1] Movement
  (`self.AddControllerYawInput` AxisValue))

(event `self.ResetCombo`
  ;[1 1 1] Animation Cancelling
  (`self.Server_EndAbility`))

(event `InputAxis|LookUp`
  (params (AxisValue :type "Float (single-precision)"))
  ;[1 1 1] Movement
  (`self.AddControllerPitchInput` AxisValue))

(event `self.NextAction`
  (bind _returnvalue (`SkeletalMeshComponent.GetAnimInstance` (`self.Mesh`)))
  ;[1 1 1] Animation Cancelling
  (set `self.IsAttacking` false)
  (set `self.CanCancel` true)
  ;[1 1 1] During next action, start blending out the currently playing animation and disable root motion so that the player can direct their roll
  (if (`self.IsMovementKeyDown`)
    (`AnimInstance.SetRootMotionMode` _returnvalue "IgnoreRootMotion")
    (`AnimInstance.StopSlotAnimation` _returnvalue 0.5 "None")
    (`KismetSystemLibrary.Delay` 0.1)
    (`AnimInstance.SetRootMotionMode` _returnvalue "RootMotionFromMontagesOnly")
    (if (`AnimInstance.IsAnyMontagePlaying` (`SkeletalMeshComponent.GetAnimInstance` (`self.Mesh`))) :!label _label
      (`KismetSystemLibrary.RetriggerableDelay` 0.2)
      (goto _label)
      (else
        (`self.Server_EndAbility`)
        (set `self.IsFullBody` false)))))

(event `InputAxis|MoveForward`
  (params (AxisValue :type "Float (single-precision)"))
  (bind (_returnvalue_roll _returnvalue_pitch _returnvalue_yaw) (`KismetMathLibrary.BreakRotator` (`self.GetControlRotation`)))
  ;[1 1 1] Movement
  (if (`self.CanMove`)
    (`self.AddMovementInput` (`KismetMathLibrary.GetForwardVector` (`KismetMathLibrary.MakeRotator` 0.0 0.0 _returnvalue_yaw)) AxisValue)
    ;[1 0 0] Get If Movement Key Down (Is a tick event)
    (if (or (!= (`self.GetInputAxisValue`) 0.0) (!= (`self.GetInputAxisValue`) 0.0)) :!label _label_2
      (set `self.IsMovementKeyDown` true)
      (else
        (set `self.IsMovementKeyDown` false)))))

(event `InputAxis|MoveRight`
  (params (AxisValue :type "Float (single-precision)"))
  (bind (_returnvalue_roll _returnvalue_pitch _returnvalue_yaw) (`KismetMathLibrary.BreakRotator` (`self.GetControlRotation`)))
  ;[1 1 1] Movement
  (if (`self.CanMove`)
    (`self.AddMovementInput` (`KismetMathLibrary.GetRightVector` (`KismetMathLibrary.MakeRotator` 0.0 0.0 _returnvalue_yaw)) AxisValue)
    (goto _label_2)))

(event `InputAction|Sprint`
  (params (Key :type "Key Structure"))
  ;[1 1 1] Sprint
  (:`Pressed`
    (if (not (`self.IsBlocking`))
      (`self.F_SprintSwitch` true)))
  (:`Released`
    (`self.F_SprintSwitch` false)))

(event `InputAction|Block`
  (params (Key :type "Key Structure"))
  ;[1 1 1] Block
  (:`Pressed`
    (if (not (`self.IsBlocking`))
      (set `self.CanMove` false)
      (`self.Server_Block` true)
      (`AbilitySystemComponent.BP_ApplyGameplayEffectToSelf` :`self` (`self.AbilitySystemComponent`) :`GameplayEffectClass` "/Game/_Main/Characters/GameplayAbilities/GeneralGameplayEffects/GE_Block.GE_Block_C")))
  (:`Released`
    (set `self.CanMove` true)
    (`self.Server_Block` false)
    (`AbilitySystemComponent.RemoveActiveGameplayEffectBySourceEffect` (`self.AbilitySystemComponent`) "/Game/_Main/Characters/GameplayAbilities/GeneralGameplayEffects/GE_Block.GE_Block_C" null -1)))

(event `InputAction|UseItem`
  (params (Key :type "Key Structure"))
  ;[1 1 1] Healing
  (:`Pressed`
    (if (and (not (`self.IsAttacking`)) (not (`self.IsRolling`)))
      (`AbilitySystemComponent.TryActivateAbilityByClass` (`self.AbilitySystemComponent`) "/Game/_Main/Characters/GameplayAbilities/Potion/GA_Potion.GA_Potion_C" true))))

(event `Server_ToggleSprint`
  (params (State :type Boolean))
  ;[1 1 1] Sprint
  (`self.F_SprintSwitch` State))

(event `Server_Block`
  (params (State :type Boolean))
  ;[1 1 1] Block
  (if State
    (set `self.IsBlocking` true)
    (else
      (set `self.IsBlocking` false))))

(event `InputAction|Dodge`
  (params (Key :type "Key Structure"))
  ;[1 1 1] Roll
  (:`Pressed`
    (if (and (not (`self.IsAttacking`)) (not (`self.IsRolling`)) (`self.CanMove`))
      (bind _returnvalue (`AbilitySystemComponent.TryActivateAbilityByClass` (`self.AbilitySystemComponent`) "/Game/_Main/Characters/GameplayAbilities/Dodge/GA_Dodge.GA_Dodge_C" true))
      (if _returnvalue
        (set `self.IsRolling` true)
        (set `self.LightComboCount` 1)
        (`KismetSystemLibrary.Delay` 1.0)
        (set `self.IsRolling` false)))))

(event `InputAction|ToggleInventory`
  (params (Key :type "Key Structure"))
  ;[1 1 1] Toggle Inventory
  (:`Pressed`
    (message `/Game/_Main/Interfaces/INT_PlayerController.ToggleInventory` (`GameplayStatics.GetPlayerController` 0))))

(event `InputAction|LightAttack`
  (params (Key :type "Key Structure"))
  ;[1 1 1] Attack
  (:`Pressed`
    (if (and (not (`self.IsRolling`)) (`self.CanMove`) (not (`self.IsAttacking`)))
      (bind _returnvalue (`AbilitySystemComponent.TryActivateAbilityByClass` (`self.AbilitySystemComponent`) "/Game/_Main/Characters/GameplayAbilities/Melee/GA_Melee.GA_Melee_C" true))
      (if _returnvalue
        (set `self.IsAttacking` true)
        (set `self.IsFullBody` true)))))

(event `InputAction|HeavyAttack`
  (params (Key :type "Key Structure"))
  ;[1 1 1] Attack
  (:`Pressed`
    (if (and (not (`self.IsRolling`)) (`self.CanMove`) (not (`self.IsAttacking`)))
      (bind _returnvalue (`AbilitySystemComponent.TryActivateAbilityByClass` (`self.AbilitySystemComponent`) "/Game/_Main/Characters/GameplayAbilities/HeavyAttack/GA_HeavyAttack.GA_HeavyAttack_C" true))
      (if _returnvalue
        (set `self.IsAttacking` true)
        (set `self.IsFullBody` true)))))

(event `Server_EndAbility`
  ;[1 1 1] Attack
  (set `self.IsAttacking` false)
  (set `self.CanCancel` false)
  (set `self.LightComboCount` 1))

(event `self.LightAttack`
  ;[1 1 1] Attack
  (`/Engine/EditorBlueprintResources/ActorMacros.Switch Has Authority`
    (:`Authority`
      (bind _outactors (`KismetSystemLibrary.SphereOverlapActors` (+ (`self.K2_GetActorLocation`) (* (`self.GetActorForwardVector`) (`self.DistanceSphereOverlap`))) 100.0 (`|MakeArray` "ObjectTypeQuery3" :!type "EObjectTypeQuery Enum") "/Game/_Main/BaseClasses/BP_CharacterBase.BP_CharacterBase_C" (`|MakeArray` self :!type "Actor Object Reference")))
      (for _array_element _outactors
        (`AbilitySystemBlueprintLibrary.SendGameplayEventToActor` self (struct :`TagName` "skill.melee.dealDamage") (make `GameplayEventData` (struct) self _array_element))))))

(event `self.PlayBossEntrance`
  (params (IsPaused :type Boolean) (BossName :type Text))
  ;[1 1 1] Play Boss Entrance and Toggle Boss Info Overlay
  (if IsPaused
    (set `self.CanMove` false)
    (else
      (set `self.CanMove` true)
      (message `/Game/_Main/Interfaces/INT_PlayerController.ToggleBossInfoOverlay` (`self.GetController`) "Visible" BossName))))

(event `self.BP_OnHealthChanged`
  (params (Health :type "Float (single-precision)") (MaxHealth :type "Float (single-precision)"))
  ;[1 1 1] Update UI on Resource Change
  (message `/Game/_Main/Interfaces/INT_PlayerController.UpdateHealthUI` (`self.GetController`) (/ Health MaxHealth)))

(event `self.BP_OnManaChanged`
  (params (Mana :type "Float (single-precision)") (MaxMana :type "Float (single-precision)"))
  ;[1 1 1] Update UI on Resource Change
  (message `/Game/_Main/Interfaces/INT_PlayerController.UpdateManaUI` (`self.GetController`) (/ Mana MaxMana)))

(event `self.BP_OnStaminaChanged`
  (params (Stamina :type "Float (single-precision)") (MaxStamina :type "Float (single-precision)"))
  ;[1 1 1] Update UI on Resource Change
  (message `/Game/_Main/Interfaces/INT_PlayerController.UpdateStaminaUI` (`self.GetController`) (/ Stamina MaxStamina)))

(event `self.BP_Death`
  ;[1 1 1] Death
  (if (not (`self.PlayerDead`))
    (set `self.IsFullBody` true)
    (set `self.PlayerDead` true)
    (`self.UpdateMovement` false)
    (message `/Game/_Main/Interfaces/INT_PlayerController.DeathScreen` (`self.GetController`))
    (`GameAnalytics.AddDesignEvent` "PlayerDead")))

(event `self.SetPickupInfo`
  (params (PickupActor :type "/Game/_Main/Interactables/BP_BasePickup Object Reference") (IsOverlapping :type Boolean))
  (bind _returnvalue (`self.GetController`))
  ;[1 1 1] Pickup Info
  (if IsOverlapping
    (bind _output_get (set `self.OverlappedPickup` PickupActor))
    (message `/Game/_Main/Interfaces/INT_PlayerController.ShowPickupName` _returnvalue true (`KismetTextLibrary.Conv_NameToText` (`.Name_18_D0186B6F4758389A94E4EDB0A5287F40` (break `/Game/_Main/Inventory/Structs/ST_ItemData` (`/Game/_Main/Interactables/BP_BasePickup.Information` _output_get)))))
    (else
      (set `self.OverlappedPickup` PickupActor)
      (message `/Game/_Main/Interfaces/INT_PlayerController.ShowPickupName` _returnvalue false ""))))

(event `InputAction|Interact`
  (params (Key :type "Key Structure"))
  ;[1 1 1] Pickup
  (:`Pressed`
    (`self.Server_InteractWithObject`)))

(event `Server_InteractWithObject`
  ;[1 1 1] Pickup
  (`self.OverlappedPickup`
    (:`then`
      (`self.HandlePickup`))
    (:`else`)))

(event `HandlePickup`
  (bind _overlappedpickup (`self.OverlappedPickup`))
  (bind _information (`/Game/_Main/Interactables/BP_BasePickup.Information` _overlappedpickup))
  ;[1 1 1] Pickup
  (bind _successfullyadded (`/Game/_Main/Inventory/Libraries/BPFL_Inventory.AddItem` _information (`.Quantity_25_B13D754F4E7733204E0E0CB9572D03DC` (break `/Game/_Main/Inventory/Structs/ST_ItemData` _information))))
  (if _successfullyadded
    (`GameAnalytics.AddDesignEventWithValue` "Pickup" 1.0)
    (`self.K2_DestroyActor` _overlappedpickup)))

(event `self.OnEnemyDeath`
  (`AbilitySystemComponent.BP_ApplyGameplayEffectToSelf` :`self` (`self.AbilitySystemComponent`) :`GameplayEffectClass` "/Game/_Main/Characters/GameplayAbilities/GeneralGameplayEffects/GE_ManaOnKill.GE_ManaOnKill_C"))

(fn `F_CalculateControlFacingDirection`
  (returns (ControllerDirection :type "Float (double-precision)"))
  (return (`AnimInstance.CalculateDirection` (`SkeletalMeshComponent.GetAnimInstance` (`self.Mesh`)) (`KismetMathLibrary.GetForwardVector` (`self.GetControlRotation`)) (`KismetMathLibrary.MakeRotator` 0.0))))

(fn `F_DetermineHeavyCombo`
  (returns (MontageToPlay :type "AnimMontage Object Reference"))
  (switch `int` (`self.LightComboCount`)
    (:`1`
      (bind _output_get (set `self.MeleeMontage` "/Game/_Main/Animations/Longsword/Longsword_Heavy_Combo1_Montage.Longsword_Heavy_Combo1_Montage"))
      (`/Engine/EditorBlueprintResources/StandardMacros.IncrementInt` (`self.LightComboCount`)
        (:`  `
          (set `self.MeleeComboDamageLevel` 1)
          (return _output_get))))
    (:`2`
      (bind _output_get_2 (set `self.MeleeMontage` "/Game/_Main/Animations/Longsword/Longsword_Heavy_Combo2_Montage.Longsword_Heavy_Combo2_Montage"))
      (`/Engine/EditorBlueprintResources/StandardMacros.IncrementInt` (`self.LightComboCount`)
        (:`  `
          (set `self.MeleeComboDamageLevel` 2)
          (return _output_get_2))))
    (:`3`
      (bind _output_get_3 (set `self.MeleeMontage` "/Game/_Main/Animations/Longsword/Longsword_Heavy_Combo3_Montage.Longsword_Heavy_Combo3_Montage"))
      (`/Engine/EditorBlueprintResources/StandardMacros.IncrementInt` (`self.LightComboCount`)
        (:`  `
          (set `self.MeleeComboDamageLevel` 3)
          (return _output_get_3))))
    (:`4`
      (bind _output_get_4 (set `self.MeleeMontage` "/Game/_Main/Animations/Longsword/Longsword_Heavy_Combo4_Montage.Longsword_Heavy_Combo4_Montage"))
      (set `self.LightComboCount` 1)
      (set `self.MeleeComboDamageLevel` 4)
      (return _output_get_4))
    (:`5`
      (bind _output_get_5 (set `self.MeleeMontage` "/Game/_Main/Animations/Longsword/Longsword_Heavy_Combo4_Montage.Longsword_Heavy_Combo4_Montage"))
      (set `self.LightComboCount` 1)
      (set `self.MeleeComboDamageLevel` 4)
      (return _output_get_5))))

(fn `F_DetermineLightCombo`
  (returns (MontageToPlay :type "AnimMontage Object Reference"))
  (switch `int` (`self.LightComboCount`)
    (:`1`
      (bind _output_get (set `self.MeleeMontage` "/Game/_Main/Animations/Longsword/Longsword_Combo1_Montage.Longsword_Combo1_Montage"))
      (`/Engine/EditorBlueprintResources/StandardMacros.IncrementInt` (`self.LightComboCount`)
        (:`  `
          (set `self.MeleeComboDamageLevel` 1)
          (return _output_get))))
    (:`2`
      (bind _output_get_2 (set `self.MeleeMontage` "/Game/_Main/Animations/Longsword/Longsword_Combo2_Montage.Longsword_Combo2_Montage"))
      (`/Engine/EditorBlueprintResources/StandardMacros.IncrementInt` (`self.LightComboCount`)
        (:`  `
          (set `self.MeleeComboDamageLevel` 2)
          (return _output_get_2))))
    (:`3`
      (bind _output_get_3 (set `self.MeleeMontage` "/Game/_Main/Animations/Longsword/Longsword_Combo3_Montage.Longsword_Combo3_Montage"))
      (`/Engine/EditorBlueprintResources/StandardMacros.IncrementInt` (`self.LightComboCount`)
        (:`  `
          (set `self.MeleeComboDamageLevel` 3)
          (return _output_get_3))))
    (:`4`
      (bind _output_get_4 (set `self.MeleeMontage` "/Game/_Main/Animations/Longsword/Longsword_Combo4_Montage.Longsword_Combo4_Montage"))
      (`/Engine/EditorBlueprintResources/StandardMacros.IncrementInt` (`self.LightComboCount`)
        (:`  `
          (set `self.MeleeComboDamageLevel` 4)
          (return _output_get_4))))
    (:`5`
      (bind _output_get_5 (set `self.MeleeMontage` "/Game/_Main/Animations/Longsword/Longsword_Combo5_Montage.Longsword_Combo5_Montage"))
      (set `self.LightComboCount` 1)
      (set `self.MeleeComboDamageLevel` 5)
      (return _output_get_5))))

(fn `F_Dodge`
  (`self.LaunchCharacter` (`GameplayStatics.GetPlayerCharacter` 0) (* (`KismetMathLibrary.GetForwardVector` (`KismetMathLibrary.MakeRotator` (.roll (`SceneComponent.K2_GetComponentRotation` (`self.Mesh`))) (.pitch (`SceneComponent.K2_GetComponentRotation` (`self.Mesh`))) (+ (.yaw (`SceneComponent.K2_GetComponentRotation` (`self.Mesh`))) 90.0))) (`self.DodgeDistance`)) true true))

(fn `F_GetPlayerInputDirection`
  (returns (PlayerMoveDirection :type "Vector Structure"))
  (return (`KismetMathLibrary.MakeVector` (`self.GetInputAxisValue`) (`self.GetInputAxisValue`))))

(fn `F_GetRollDirection`
  (returns (RollMontage :type "AnimMontage Object Reference"))
  (if (and (not (`self.IsAttacking`)) (not (`self.IsRolling`)))
    (if (or (`self.IsLockedOn`) (`self.CanCancel`))
      (if (`KismetMathLibrary.InRange_FloatFloat` (`self.F_CalculateControlFacingDirection`) 22.5 67.5 false false)
        (return "/Game/_Main/Animations/RollAndDodge/RollForwardRight_Root_Montage.RollForwardRight_Root_Montage")
        (elif (`KismetMathLibrary.InRange_FloatFloat` (`self.F_CalculateControlFacingDirection`) -22.5 -67.5 false false)
          (return "/Game/_Main/Animations/RollAndDodge/RollForwardLeft_Root_Montage.RollForwardLeft_Root_Montage")
          (elif (`KismetMathLibrary.InRange_FloatFloat` (`self.F_CalculateControlFacingDirection`) 112.5 157.5 false false)
            (return "/Game/_Main/Animations/RollAndDodge/RollBackwardRight_Root_Montage.RollBackwardRight_Root_Montage")
            (elif (`KismetMathLibrary.InRange_FloatFloat` (`self.F_CalculateControlFacingDirection`) -112.5 -157.5 false false)
              (return "/Game/_Main/Animations/RollAndDodge/RollBackwardLeft_Root_Montage.RollBackwardLeft_Root_Montage")
              (elif (`KismetMathLibrary.InRange_FloatFloat` (`self.F_CalculateControlFacingDirection`) -22.5 22.5)
                (return "/Game/_Main/Animations/RollAndDodge/RollForward_Root_Montage.RollForward_Root_Montage")
                (elif (>= (`KismetMathLibrary.Abs` (`self.F_CalculateControlFacingDirection`)) 157.5)
                  (return "/Game/_Main/Animations/RollAndDodge/RollBackward_Root_Montage.RollBackward_Root_Montage")
                  (elif (`KismetMathLibrary.InRange_FloatFloat` (`self.F_CalculateControlFacingDirection`) 67.5 112.5)
                    (return "/Game/_Main/Animations/RollAndDodge/RollRight_Root_Montage.RollRight_Root_Montage")
                    (elif (`KismetMathLibrary.InRange_FloatFloat` (`self.F_CalculateControlFacingDirection`) -67.5 -112.5)
                      (return "/Game/_Main/Animations/RollAndDodge/RollLeft_Root_Montage.RollLeft_Root_Montage")
                      (else
                        (return null))))))))))
      (else
        (return "/Game/_Main/Animations/RollAndDodge/RollForward_Root_Montage.RollForward_Root_Montage")))
    (else
      (return null))))

(fn `F_SprintSwitch`
  (params (SprintState :type Boolean))
  (locals (LocalSprint :type Boolean))
  (set `local.LocalSprint` SprintState)
  (`/Engine/EditorBlueprintResources/ActorMacros.Switch Has Authority`
    (:`Authority`
      (if (`local.LocalSprint`)
        (set `CharacterMovementComponent.MaxWalkSpeed` (`self.SprintSpeed`) (`self.CharacterMovement`))
        (set `self.IsSprinting` true)
        (else
          (set `CharacterMovementComponent.MaxWalkSpeed` (`self.JogSpeed`) (`self.CharacterMovement`))
          (set `self.IsSprinting` false)))
      (return))
    (:`Remote`
      (`self.Server_ToggleSprint` (`local.LocalSprint`))
      (if (`local.LocalSprint`)
        (set `CharacterMovementComponent.MaxWalkSpeed` (`self.SprintSpeed`) (`self.CharacterMovement`))
        (else
          (set `CharacterMovementComponent.MaxWalkSpeed` (`self.JogSpeed`) (`self.CharacterMovement`))))
      (return))))

(fn `IsDead`
  (returns (Dead :type Boolean))
  (return (`self.PlayerDead`)))

(fn `OnRep_IsBlocking`
  (bind _returnvalue (`SkeletalMeshComponent.GetAnimInstance` (`self.Mesh`)))
  (if (`self.IsBlocking`)
    (message `/Game/_Main/Interfaces/INT_PlayerAnimBp.BlockingState` _returnvalue true)
    (else
      (message `/Game/_Main/Interfaces/INT_PlayerAnimBp.BlockingState` _returnvalue false))))

(fn `OnRep_IsDead`
  (if (`self.PlayerDead`)
    (`SkeletalMeshComponent.PlayAnimation` (`self.Mesh`) "/Game/_Main/Animations/Anim_DieA.Anim_DieA" false)
    (`PrimitiveComponent.SetCollisionProfileName` (`self.CapsuleComponent`) "None" true)))

(fn `OnRep_IsFullBody`
  (bind _returnvalue (`SkeletalMeshComponent.GetAnimInstance` (`self.Mesh`)))
  (if (`self.IsFullBody`)
    (message `/Game/_Main/Interfaces/INT_PlayerAnimBp.FullBodyState` _returnvalue true)
    (else
      (message `/Game/_Main/Interfaces/INT_PlayerAnimBp.FullBodyState` _returnvalue false))))

(fn `OnRep_IsLockedOn`)

(fn `OnRep_IsRolling`
  (bind _returnvalue (`SkeletalMeshComponent.GetAnimInstance` (`self.Mesh`)))
  (if (`self.IsRolling`)
    (message `/Game/_Main/Interfaces/INT_PlayerAnimBp.RollingState` _returnvalue true)
    (else
      (message `/Game/_Main/Interfaces/INT_PlayerAnimBp.RollingState` _returnvalue false))))

(fn `OnRep_IsSprinting`
  (bind _returnvalue (`SkeletalMeshComponent.GetAnimInstance` (`self.Mesh`)))
  (if (`self.IsSprinting`)
    (message `/Game/_Main/Interfaces/INT_PlayerAnimBp.SprintState` _returnvalue true)
    (else
      (message `/Game/_Main/Interfaces/INT_PlayerAnimBp.SprintState` _returnvalue false))))

(fn `PlayerRef`
  (returns (PlayerRef :type "/Game/_Main/Characters/BP_PlayerCharacter Object Reference"))
  (return self))

(fn `UpdateMovement`
  (params (CanMove :type Boolean))
  (returns (Return :type Boolean))
  (bind _output_get (set `self.CanMove` CanMove))
  (return _output_get))

(fn `UserConstructionScript`
  (`parent.UserConstructionScript`))