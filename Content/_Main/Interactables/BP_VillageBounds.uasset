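; BP_VillageBounds is a trigger volume that switches background music as the player enters or leaves the village.
; On BeginPlay it spawns persistent 2D sounds for the village and outside cues, then deactivates both.
; Player overlap begin and end events on the collision component activate one track and deactivate the other with a reset.
; Neither track is reactivated until the first overlap event fires.
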(event `self.ReceiveBeginPlay`
  (bind _returnvalue (`GameplayStatics.SpawnSound2D` "/Game/_Main/Audio/BGM/Cue_VillageOutside.Cue_VillageOutside" 1.0 1.0 0.0 null false false))
  (bind _output_get (set `self.BGM_VillageOutside` _returnvalue))
  (bind _returnvalue_2 (`GameplayStatics.SpawnSound2D` "/Game/_Main/Audio/BGM/Cue_Village.Cue_Village" 1.0 1.0 0.0 null false false))
  (bind _output_get_2 (set `self.BGM_Village` _returnvalue_2))
  (`ActorComponent.SetActive` _output_get_2 false false)
  (`ActorComponent.SetActive` _output_get false false))

(event `self.CollisionComponent.OnComponentBeginOverlap`
  (params (OverlappedComponent :type "PrimitiveComponent Object Reference") (OtherActor :type "Actor Object Reference") (OtherComp :type "PrimitiveComponent Object Reference") (OtherBodyIndex :type Integer) (bFromSweep :type Boolean) (SweepResult :type "HitResult Structure (by ref)"))
  (cast `/Game/_Main/Characters/BP_PlayerCharacter` OtherActor)
  (`ActorComponent.SetActive` (`self.BGM_VillageOutside`) false true)
  (`ActorComponent.SetActive` (`self.BGM_Village`) true true))

(event `self.CollisionComponent.OnComponentEndOverlap`
  (params (OverlappedComponent :type "PrimitiveComponent Object Reference") (OtherActor :type "Actor Object Reference") (OtherComp :type "PrimitiveComponent Object Reference") (OtherBodyIndex :type Integer))
  (cast `/Game/_Main/Characters/BP_PlayerCharacter` OtherActor)
  (`ActorComponent.SetActive` (`self.BGM_Village`) false true)
  (`ActorComponent.SetActive` (`self.BGM_VillageOutside`) true true))

(fn `UserConstructionScript`)