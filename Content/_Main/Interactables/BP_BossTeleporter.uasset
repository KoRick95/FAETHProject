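; BP_BossTeleporter is an interactable trigger that teleports the player to a BP_TeleportDestination actor, likely for boss encounters given its name.
; On BeginPlay it caches the first BP_TeleportDestination found in the level.
; When its collision component is overlapped, it gets the player reference through a message call, moves that player to the destination's location, and sets the controller's rotation to the destination's facing.
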(event `self.ReceiveBeginPlay`
  (bind _returnvalue (`GameplayStatics.GetActorOfClass` "/Game/_Main/Interactables/BP_TeleportDestination.BP_TeleportDestination_C"))
  (set `self.TeleportDestination` _returnvalue))

(event `self.CollisionComponent.OnComponentBeginOverlap`
  (params (OverlappedComponent :type "PrimitiveComponent Object Reference") (OtherActor :type "Actor Object Reference") (OtherComp :type "PrimitiveComponent Object Reference") (OtherBodyIndex :type Integer) (bFromSweep :type Boolean) (SweepResult :type "HitResult Structure (by ref)"))
  (bind _teleportdestination (`self.TeleportDestination`))
  (bind _playerref (message `/Game/_Main/Interfaces/INT_PlayerCharacter.PlayerRef` OtherActor))
  (`/Engine/EditorBlueprintResources/StandardMacros.IsValid` _playerref
    (:`Is Valid`
      (`self.K2_TeleportTo` :`self` _playerref :`DestLocation` (`self.K2_GetActorLocation` _teleportdestination))
      (`Controller.SetControlRotation` (`GameplayStatics.GetPlayerController` 0) (`self.K2_GetActorRotation` _teleportdestination)))))

(fn `UserConstructionScript`)