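; BP_BasePickup is an interactable world pickup that configures itself from an item data table row.
; On BeginPlay it sets the mesh from that row and writes an "[E]" name to the nameplate widget.
; Collider overlaps toggle the nameplate and report the pickup to the player, with begin-overlap authority-only and end-overlap ungated.
; DisablePhysics is an empty event, and the physics and collision nodes are unwired.
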(event `self.ReceiveBeginPlay`
  (bind (_datatable _rowname) (break `DataTableRowHandle` (`self.Item`)))
  ;[1 1 1] Get Item Information
  (bind _returnvalue (`|GetDataTableRow` _datatable _rowname)
    (:`then`
      (set `self.Information` _returnvalue)
      (`StaticMeshComponent.SetStaticMesh` (`self.StaticMesh`) (`.Mesh_23_10FFC57542DBA7584D6692A4294EA3D3` (break `/Game/_Main/Inventory/Structs/ST_ItemData` (`self.Information`))))
      ;[1 1 1] Update Nameplate
      (`TextBlock.SetText` (`/Game/_Main/Interactables/W_PickupNameplate.NameText` (cast `/Game/_Main/Interactables/W_PickupNameplate` (`WidgetComponent.GetUserWidgetObject` (`self.Nameplate`)) :!pure true)) (`KismetTextLibrary.Conv_StringToText` (`KismetStringLibrary.Concat_StrStr` "[E]" (`KismetStringLibrary.Conv_NameToString` (`.Name_18_D0186B6F4758389A94E4EDB0A5287F40` (break `/Game/_Main/Inventory/Structs/ST_ItemData` (`self.Information`))))))))))

(event `/Game/_Main/Interfaces/INT_Pickups.DisablePhysics`
  ;[1 1 1] Disable Physics
)

(event `self.InteractionCollider.OnComponentBeginOverlap`
  (params (OverlappedComponent :type "PrimitiveComponent Object Reference") (OtherActor :type "Actor Object Reference") (OtherComp :type "PrimitiveComponent Object Reference") (OtherBodyIndex :type Integer) (bFromSweep :type Boolean) (SweepResult :type "HitResult Structure (by ref)"))
  ;[1 1 1] On player enter
  (`/Engine/EditorBlueprintResources/ActorMacros.Switch Has Authority`
    (:`Authority`
      (if (`self.ActorHasTag` OtherActor "Player")
        (`SceneComponent.SetVisibility` (`self.Nameplate`) true false)
        (message `/Game/_Main/Interfaces/INT_PlayerCharacter.SetPickupInfo` OtherActor self true)))))

(event `self.InteractionCollider.OnComponentEndOverlap`
  (params (OverlappedComponent :type "PrimitiveComponent Object Reference") (OtherActor :type "Actor Object Reference") (OtherComp :type "PrimitiveComponent Object Reference") (OtherBodyIndex :type Integer))
  ;[1 1 1] On player exit
  (if (`KismetMathLibrary.ClassIsChildOf` (`GameplayStatics.GetObjectClass` OtherActor) "/Game/_Main/Characters/BP_PlayerCharacter.BP_PlayerCharacter_C")
    (`SceneComponent.SetVisibility` (`self.Nameplate`) false false)
    (message `/Game/_Main/Interfaces/INT_PlayerCharacter.SetPickupInfo` OtherActor self false)))

(fn `UserConstructionScript`)