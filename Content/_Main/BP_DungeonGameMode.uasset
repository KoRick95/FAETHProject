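; Game mode for a multiplayer procedural dungeon that seeds generation and spawns players.
; After a join delay it picks a random seed and sends it to queued controllers so each client builds its own dungeon.
; When initial streamed chunks load, it spawns and possesses characters at the first PlayerStart.
; Match start waits for initialisation and all players ready, then respawns PlayerStarts with small random offsets around the first.
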(event `self.ReceiveBeginPlay`
  (set `self.NumPlayersReady` 0)
  ;[1 1 1] Wait for players to join
  (`KismetSystemLibrary.Delay` 3.0)
  (set `self.DungeonSeed` (`KismetMathLibrary.RandomInteger` 10000000))
  ;[1 1 1] Setup Level Streaming
  (bind _returnvalue (`GameplayStatics.GetActorOfClass` "/Script/DungeonArchitectRuntime.Dungeon"))
  (bind _output_get (set `self.Dungeon` _returnvalue))
  (`/Engine/EditorBlueprintResources/StandardMacros.IsValid` _output_get
    (:`Is Valid`
      (add `DungeonLevelStreamingModel.OnInitialChunksLoaded` (`Dungeon.LevelStreamingModel` _output_get) (delegate `OnSpawnRoomsLoaded`))
      ;[1 1 1] Randomise Dungeon
      (set `DungeonConfig.Seed` (`self.DungeonSeed`) (`Dungeon.Config` (`self.Dungeon`)))
      ;[1 1 1] Have each client build their own dungeon from the provided seed
      (for _array_element (`self.PendingClients`)
        (bind _asbp_player_controller (cast `/Game/_Main/BP_PlayerController` _array_element))
        (`/Game/_Main/BP_PlayerController.Client_BuildDungeon` _asbp_player_controller (`self.DungeonSeed`))))))

(event `OnSpawnRoomsLoaded`
  (params (Dungeon :type "Dungeon Object Reference"))
  ;[1 1 1] When Spawn Room Loaded, Assign Pawn
  (set `self.ServerDungeonReady` true)
  (bind _outactors (`GameplayStatics.GetAllActorsOfClass` "/Script/Engine.PlayerStart"))
  (set `self.SpawnPoints` _outactors)
  (`KismetSystemLibrary.Delay` 1.0)
  (`self.AssignPawn`))

(event `self.K2_PostLogin`
  (params (NewPlayer :type "PlayerController Object Reference"))
  (`KismetArrayLibrary.Array_Add` (`self.PendingClients`) NewPlayer))

(event `self.AssignPawn`
  (bind _returnvalue (`self.GetTransform` (`|GetArrayItem` (`self.SpawnPoints`))))
  (for _array_element (`self.PendingClients`)
    (bind _returnvalue_2 (`|SpawnActorFromClass` "/Game/_Main/Characters/BP_PlayerCharacter.BP_PlayerCharacter_C" _returnvalue "Undefined" "OverrideRootScale" null null))
    (`self.K2_TeleportTo` _array_element (.location _returnvalue) (.rotation _returnvalue))
    (`Controller.Possess` _array_element _returnvalue_2)
    (`self.UnloadSplashScreen`))
  (set `self.GameInitialised` true)
  (`KismetArrayLibrary.Array_Clear` (`self.PendingClients`)))

(fn `F_InitialisePlayerStart`
  (locals (PreferredSpawnLocation :type "Vector Structure"))
  (bind _outactors (`GameplayStatics.GetAllActorsOfClass` "/Script/Engine.PlayerStart"))
  (bind _output_get (set `local.PreferredSpawnLocation` (`self.K2_GetActorLocation` (`|GetArrayItem` _outactors))))
  (for _array_element _outactors
    (`self.K2_DestroyActor` _array_element)
    (`|SpawnActorFromClass` "/Script/Engine.PlayerStart" (`KismetMathLibrary.Conv_VectorToTransform` (+ _output_get (* (`KismetMathLibrary.Normal` (* (`KismetMathLibrary.RandomUnitVector`) (1.0 1.0 0.0))) 50.0))) "AdjustIfPossibleButAlwaysSpawn" "OverrideRootScale" null null)))

(fn `F_NotifyPlayerReady`
  (`/Engine/EditorBlueprintResources/StandardMacros.IncrementInt` (`self.NumPlayersReady`)))

(fn `ReadyToStartMatch`
  (returns (ReturnValue :type Boolean))
  ;[1 1 1] Wait until all players loaded
  (bind _returnvalue (`self.GetNumPlayers`))
  (bind _returnvalue_2 (and (>= (`self.NumPlayersReady`) _returnvalue) (`self.GameInitialised`)))
  (if _returnvalue_2
    (`self.F_InitialisePlayerStart`))
  (return _returnvalue_2))

(fn `UserConstructionScript`)