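; Base enemy AI character handling melee hits, health display, death and loot.
; A toggleable melee sphere or an authority-only forward sphere overlap finds Player-tagged actors and sends a Gameplay Ability System damage event to itself.
; Health changes update an overhead bar, or the player's boss bar for bosses.
; Death plays an empty, overridable animation hook, disables movement, drops random loot through the player's inventory, notifies the player, then destroys the actor.
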(event `self.ReceiveBeginPlay`
  (bind _health (`self.Health`))
  (`Widget.SetVisibility` (`WidgetComponent.GetUserWidgetObject` (`self.HealthBar`)) "Collapsed")
  (`self.SetMaxHealth` _health)
  (`self.SetHealth` _health))

(event `/Game/_Main/Interfaces/INT_EnemyAI.SetMeleeCollision`
  (params (State :type Boolean))
  (bind _meleesphere (`self.MeleeSphere`))
  ;[1 1 1] Use Melee Sphere to Damage
  (if State
    (`PrimitiveComponent.SetCollisionEnabled` _meleesphere "QueryOnly")
    (else
      (`PrimitiveComponent.SetCollisionEnabled` _meleesphere "NoCollision"))))

(event `self.MeleeSphere.OnComponentBeginOverlap`
  (params (OverlappedComponent :type "PrimitiveComponent Object Reference") (OtherActor :type "Actor Object Reference") (OtherComp :type "PrimitiveComponent Object Reference") (OtherBodyIndex :type Integer) (bFromSweep :type Boolean) (SweepResult :type "HitResult Structure (by ref)"))
  ;[1 1 1] Use Melee Sphere to Damage
  (if (`self.ActorHasTag` OtherActor "Player")
    (`AbilitySystemBlueprintLibrary.SendGameplayEventToActor` self (struct :`TagName` "skill.melee.dealDamage") (make `GameplayEventData` (struct) self OtherActor))))

(event `/Game/_Main/Interfaces/INT_EnemyAI.DoSphereOverlap`
  ;[1 1 1] Create Melee Sphere to Deal Damage
  (`self.F_DoSphereOverlap` 100.0 200.0))

(event `self.BP_Death`
  ;[1 1 1] Death
  (if (not (`self.IsDead`))
    (set `self.IsDead` true)
    (`self.Multi_DeathAnimation`)
    (`self.DetachFromControllerPendingDestroy`)
    (`CharacterMovementComponent.SetAvoidanceEnabled` (`self.CharacterMovement`) false)
    (`CharacterMovementComponent.DisableMovement` (`self.CharacterMovement`))
    (`self.DropLoot`)
    (message `/Game/_Main/Interfaces/INT_PlayerCharacter.OnEnemyDeath` (`GameplayStatics.GetPlayerCharacter` 0))
    (`KismetSystemLibrary.Delay` 5.0)
    (`self.K2_DestroyActor`)))

(event `Multi_DeathAnimation`
  ;[1 1 1] Death
  (`PrimitiveComponent.SetCollisionProfileName` (`self.CapsuleComponent`) "Ragdoll" true)
  (`SkeletalMeshComponent.SetAnimationMode` (`self.Mesh`) "AnimationSingleNode")
  (`self.F_PlayDeathAnimation`))

(event `DropLoot`
  (bind _potentiallootdrops (`self.PotentialLootDrops`))
  (bind _returnvalue (`KismetArrayLibrary.Array_Length` _potentiallootdrops))
  (bind _returnvalue_2 (`KismetMathLibrary.RandomInteger` _returnvalue))
  ;[1 1 1] Drop Loot
  (bind _playerref (message `/Game/_Main/Interfaces/INT_PlayerCharacter.PlayerRef` (`GameplayStatics.GetPlayerCharacter` 0)))
  (if (> _returnvalue 0)
    (if (< _returnvalue_2 _returnvalue)
      (`/Game/_Main/Inventory/BP_InventoryComponent.DropLoot` (`/Game/_Main/Characters/BP_PlayerCharacter.BP_InventoryComponent` _playerref) (`|GetArrayItem` _potentiallootdrops _returnvalue_2) (`SceneComponent.K2_GetComponentToWorld` (`self.CapsuleComponent`))))))

(event `self.BP_OnHealthChanged`
  (params (Health :type "Float (single-precision)") (MaxHealth :type "Float (single-precision)"))
  (bind _returnvalue (/ Health MaxHealth))
  (bind _returnvalue_2 (`WidgetComponent.GetUserWidgetObject` (`self.HealthBar`)))
  ;[1 1 1] On Health Changed
  (if (`self.IsBoss`)
    (message `/Game/_Main/Interfaces/INT_PlayerController.UpdateBossHealthBar` (`GameplayStatics.GetPlayerController` 0) _returnvalue)
    (else
      (`/Game/_Main/UI/WBP_HealthBar.SetPercentage` (cast `/Game/_Main/UI/WBP_HealthBar` _returnvalue_2 :!pure true) _returnvalue)
      (if (not (`Widget.IsVisible` _returnvalue_2))
        (`Widget.SetVisibility` _returnvalue_2 "Visible")))))

(event `/Game/_Main/Interfaces/INT_EnemyAI.ToggleTargetWidget`
  (params (State :type Boolean) (Player :type "Actor Object Reference"))
  ;[1 1 1] Toggle Targeting Widget
  (`self.Multi_ToggleTargetWidget` State Player))

(event `Multi_ToggleTargetWidget`
  (params (State :type Boolean) (Player :type "Actor Object Reference"))
  (bind _targetwidget (`self.TargetWidget`))
  ;[1 1 1] Toggle Targeting Widget
  (if (`KismetSystemLibrary.IsValid` (`self.GetInstigatorController` Player))
    (if State
      (`SceneComponent.SetHiddenInGame` _targetwidget false false)
      (else
        (`SceneComponent.SetHiddenInGame` _targetwidget true false)))))

(fn `EnemyRef`
  (returns (EnemyRef :type "/Game/_Main/AI/BP_EnemyBase Object Reference"))
  (return self))

(fn `F_DoSphereOverlap`
  (params (SphereRadius :type "Float (double-precision)") (SphereDistance :type "Float (double-precision)"))
  (`/Engine/EditorBlueprintResources/ActorMacros.Switch Has Authority`
    (:`Authority`
      (bind _outactors (`KismetSystemLibrary.SphereOverlapActors` (+ (`self.K2_GetActorLocation`) (* (`self.GetActorForwardVector`) SphereDistance)) SphereRadius (`|MakeArray` "ObjectTypeQuery3" :!type "EObjectTypeQuery Enum") null (`|MakeArray` self :!type "Actor Object Reference")))
      (for _array_element _outactors
        (if (`self.ActorHasTag` _array_element "Player")
          (`AbilitySystemBlueprintLibrary.SendGameplayEventToActor` self (struct :`TagName` "skill.melee.dealDamage") (make `GameplayEventData` (struct) self _array_element)))))))

(fn `F_PlayDeathAnimation`)

(fn `IsAIDead`
  (returns (IsDead :type Boolean))
  (return (`self.IsDead`)))

(fn `UserConstructionScript`
  (`parent.UserConstructionScript`))