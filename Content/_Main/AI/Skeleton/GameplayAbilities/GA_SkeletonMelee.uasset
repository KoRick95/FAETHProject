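; GA_SkeletonMelee is the skeleton AI's melee attack gameplay ability, playing a random montage from MeleeMontage.
; On each Skill.melee.dealDamage event, it applies GE_TrollMelee_Damage to the payload target and sends a stun hit message to player 0.
; The effect level comes from a separate random montage index roll, independent of the played animation.
; The ability ends when the montage completes, blends out, is interrupted or is cancelled.
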(event `self.K2_ActivateAbility`
  (bind _meleemontage (`self.MeleeMontage`))
  (bind (_outitem _outindex) (`KismetArrayLibrary.Array_Random` (`.AnimMontage_8_65B2149E4914E523BD307EA313E6CA97` (break `/Game/_Main/AI/Skeleton/Animations/ST_SkeletonAttacks` (`|GetArrayItem` _meleemontage (`KismetMathLibrary.RandomIntegerInRange` 0 (- (`KismetArrayLibrary.Array_Length` _meleemontage) 1)))))))
  (`parent.K2_ActivateAbility`)
  (`self.K2_CommitAbility`)
  (`AbilityTask_PlayMontageAndWait.CreatePlayMontageAndWaitProxy` "None" _outitem
    (:`then`
      (bind (_asynctaskproxy _payload) (`AbilityTask_WaitGameplayEvent.WaitGameplayEvent` (struct :`TagName` "skill.melee.dealDamage") null)
        (:`EventReceived`
          (`self.BP_ApplyGameplayEffectToTarget` (`AbilitySystemBlueprintLibrary.AbilityTargetDataFromActor` (`.Target` (break `GameplayEventData` _payload))) "/Game/_Main/AI/Troll/GameplayAbilities/TrollMelee/GE_TrollMelee_Damage.GE_TrollMelee_Damage_C" _outindex)
          (message `/Game/_Main/Interfaces/INT_PlayerCharacter.PlayerHit` (`GameplayStatics.GetPlayerCharacter` 0) false 1.0 (0.0 0.0 0.0)))))
    (:`OnCompleted`
      (`self.K2_EndAbility` :!label _label))
    (:`OnBlendOut`
      (goto _label))
    (:`OnInterrupted`
      (goto _label))
    (:`OnCancelled`
      (goto _label))))