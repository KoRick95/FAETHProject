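; GA_TrollMelee is the troll's melee attack gameplay ability.
; It commits, plays the light swing montage, then waits for a Skill.melee.dealDamage gameplay event to apply the GE_TrollMelee_Damage effect.
; The event handler also prints the name of the player reference obtained from the payload target, apparently for debugging.
; The ability ends when the montage completes, blends out, is interrupted or is cancelled.
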(event `self.K2_ActivateAbility`
  (`parent.K2_ActivateAbility`)
  (`self.K2_CommitAbility`)
  (`AbilityTask_PlayMontageAndWait.CreatePlayMontageAndWaitProxy` "None" "/Game/_Main/AI/Troll/Troll_LightSwing_Montage.Troll_LightSwing_Montage"
    (:`then`
      (bind (_asynctaskproxy _payload) (`AbilityTask_WaitGameplayEvent.WaitGameplayEvent` (struct :`TagName` "skill.melee.dealDamage") null)
        (:`EventReceived`
          (`self.BP_ApplyGameplayEffectToTarget` (struct) "/Game/_Main/AI/Troll/GameplayAbilities/GE_TrollMelee_Damage.GE_TrollMelee_Damage_C")
          (bind _playerref (message `/Game/_Main/Interfaces/INT_PlayerCharacter.PlayerRef` (`.Target` (break `GameplayEventData` _payload))))
          (`/Engine/EditorBlueprintResources/StandardMacros.IsValid` _playerref
            (:`Is Valid`
              (`KismetSystemLibrary.PrintString` (`KismetSystemLibrary.GetDisplayName` _playerref)))))))
    (:`OnCompleted`
      (`self.K2_EndAbility` :!label _label))
    (:`OnBlendOut`
      (goto _label))
    (:`OnInterrupted`
      (goto _label))
    (:`OnCancelled`
      (goto _label))))