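; Gameplay ability for the Lion Knight AI's special attack, a running slam.
; On activation it commits, plays the slam montage and waits for the melee deal-damage gameplay event.
; A received event applies the Lion Knight melee damage effect at a fixed raised level to the event's target and sends that actor a PlayerRef message.
; The ability ends when the montage completes, blends out, is interrupted or is cancelled.
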(event `self.K2_ActivateAbility`
  (`parent.K2_ActivateAbility`)
  (`self.K2_CommitAbility`)
  (`AbilityTask_PlayMontageAndWait.CreatePlayMontageAndWaitProxy` "None" "/Game/_Main/AI/LionKnight/Animations/LionKnight_RunningSlam_Montage.LionKnight_RunningSlam_Montage"
    (:`then`
      (bind (_asynctaskproxy _payload) (`AbilityTask_WaitGameplayEvent.WaitGameplayEvent` (struct :`TagName` "skill.melee.dealDamage") null)
        (:`EventReceived`
          (bind (_eventtag _instigator _target) (break `GameplayEventData` _payload))
          (`self.BP_ApplyGameplayEffectToTarget` (`AbilitySystemBlueprintLibrary.AbilityTargetDataFromActor` _target) "/Game/_Main/AI/LionKnight/GameplayAbilities/GE_LionKnightMelee_Damage.GE_LionKnightMelee_Damage_C" 4)
          (message `/Game/_Main/Interfaces/INT_PlayerCharacter.PlayerRef` _target))))
    (:`OnCompleted`
      (`self.K2_EndAbility` :!label _label))
    (:`OnBlendOut`
      (goto _label))
    (:`OnInterrupted`
      (goto _label))
    (:`OnCancelled`
      (goto _label))))