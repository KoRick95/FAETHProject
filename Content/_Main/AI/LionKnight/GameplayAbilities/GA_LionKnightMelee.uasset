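; GA_LionKnightMelee is the Lion Knight AI's melee attack gameplay ability.
; On activation it commits, plays a random melee montage and waits for a deal-damage gameplay event.
; That event applies the melee damage effect to the payload target at a separately randomized level, then calls PlayerRefMessage on the target.
; Montage completion, blend-out, interruption or cancellation ends the ability; a montage-already-playing check is left disconnected.
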(event `self.K2_ActivateAbility`
  (bind _meleemontages (`self.MeleeMontages`))
  (bind _returnvalue (`KismetMathLibrary.RandomIntegerInRange` 0 (`KismetArrayLibrary.Array_LastIndex` _meleemontages)))
  (`parent.K2_ActivateAbility`)
  (`self.K2_CommitAbility`)
  (`AbilityTask_PlayMontageAndWait.CreatePlayMontageAndWaitProxy` "None" (`|GetArrayItem` _meleemontages _returnvalue)
    (:`then`
      (bind (_asynctaskproxy _payload) (`AbilityTask_WaitGameplayEvent.WaitGameplayEvent` (struct :`TagName` "skill.melee.dealDamage") null)
        (:`EventReceived`
          (bind (_eventtag _instigator _target) (break `GameplayEventData` _payload))
          (`self.BP_ApplyGameplayEffectToTarget` (`AbilitySystemBlueprintLibrary.AbilityTargetDataFromActor` _target) "/Game/_Main/AI/LionKnight/GameplayAbilities/GE_LionKnightMelee_Damage.GE_LionKnightMelee_Damage_C" (+ _returnvalue 1))
          (message `/Game/_Main/Interfaces/INT_PlayerCharacter.PlayerRef` _target))))
    (:`OnCompleted`
      (`self.K2_EndAbility` :!label _label))
    (:`OnBlendOut`
      (goto _label))
    (:`OnInterrupted`
      (goto _label))
    (:`OnCancelled`
      (goto _label))))