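; Test Gameplay Ability for a melee attack that plays a longsword combo montage on the owning character.
; On activation it commits, prints a debug message and ends when the montage completes, blends out, is interrupted or is cancelled.
; On end it prints again and, if BP_TestCharacter has a queued attack, clears that flag and re-activates this same ability class, chaining buffered attacks.
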(event `self.K2_ActivateAbility`
  (`self.K2_CommitAbility`)
  (`KismetSystemLibrary.PrintString` "Ability activated" true true (struct :`G` 1.0 :`B` 0.066989 :`A` 1.0))
  (`AbilityTask_PlayMontageAndWait.CreatePlayMontageAndWaitProxy` "None" "/Game/_Main/Animations/Longsword/Longsword_Combo1_Montage.Longsword_Combo1_Montage"
    (:`OnCompleted`
      _)
    (:`OnBlendOut`
      _)
    (:`OnInterrupted`
      _)
    (:`OnCancelled`
      _))
  (`self.K2_EndAbility`))

(event `self.K2_OnEndAbility`
  (params (bWasCancelled :type Boolean))
  (`KismetSystemLibrary.PrintString` "Ability ended" true true (struct :`G` 0.465543 :`B` 1.0 :`A` 1.0))
  (bind _asbp_test_character (cast `/Game/_Main/Temporary/BP_TestCharacter` (`self.GetOwningActorFromActorInfo`)))
  (if (`/Game/_Main/Temporary/BP_TestCharacter.HasQueuedAttack` _asbp_test_character)
    (set `/Game/_Main/Temporary/BP_TestCharacter.HasQueuedAttack` false _asbp_test_character)
    (`AbilitySystemComponent.TryActivateAbilityByClass` (`BaseCharacter.AbilitySystemComponent` _asbp_test_character) "GA_TestAttack_C" true)))