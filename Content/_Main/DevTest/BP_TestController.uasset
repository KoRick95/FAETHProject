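; BP_TestController is a test player controller that handles basic movement and look input.
; MoveForward and MoveRight axes add movement input to the controlled pawn along the camera manager's forward and right vectors, using the full camera rotation.
; LookUp and Turn feed controller pitch and yaw.
; Disconnected nodes hold an inactive GA_TempRoll ability activation on BP_TestCharacter and an unused input-direction calculation.
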(event `InputAxis|MoveForward`
  (params (AxisValue :type "Float (single-precision)"))
  ;[1 1 1] Movement
  (`Pawn.AddMovementInput` (`self.K2_GetPawn`) (`KismetMathLibrary.GetForwardVector` (`PlayerCameraManager.GetCameraRotation` (`self.PlayerCameraManager`))) AxisValue false))

(event `InputAxis|MoveRight`
  (params (AxisValue :type "Float (single-precision)"))
  ;[1 1 1] Movement
  (`Pawn.AddMovementInput` (`self.K2_GetPawn`) (`KismetMathLibrary.GetRightVector` (`PlayerCameraManager.GetCameraRotation` (`self.PlayerCameraManager`))) AxisValue false))

(event `InputAxis|LookUp`
  (params (AxisValue :type "Float (single-precision)"))
  ;[1 1 1] Camera
  (`self.AddPitchInput` AxisValue))

(event `InputAction|Dodge`
  (params (Key :type "Key Structure")))

(event `InputAxis|Turn`
  (params (AxisValue :type "Float (single-precision)"))
  ;[1 1 1] Camera
  (`self.AddYawInput` AxisValue))

(fn `UserConstructionScript`)