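; BP_TestPlayer is a dev-test player Blueprint for inspecting the skill system and Gameplay Ability System through on-screen debug prints.
; After a short delay on BeginPlay, it prints the class of every skill in its SkillSystemComponent and whether Skill_TestSkill is valid.
; A DebugAbilities event prints the name of each ability resolved from the AbilitySystemComponent's spec handles.
; GetPlayer, IsDead and UpdateMovement are stubs returning empty or false.
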(event `self.ReceiveBeginPlay`
  (`KismetSystemLibrary.Delay` 0.2)
  (for _array_element (`SkillSystemComponent.GetAllSkills` (`self.SkillSystemComponent`))
    (`KismetSystemLibrary.PrintString` (`KismetSystemLibrary.GetClassDisplayName` (`GameplayStatics.GetObjectClass` _array_element)) true true (struct :`G` 0.66 :`B` 1.0 :`A` 1.0) 3.0))
  (`/Engine/EditorBlueprintResources/StandardMacros.IsValid` (`SkillSystemComponent.GetSkillByClass` (`self.SkillSystemComponent`) "/Game/_Main/DevTest/Skill_TestSkill.Skill_TestSkill_C")
    (:`Is Valid`
      (`KismetSystemLibrary.PrintString` "valid" true true (struct :`G` 0.66 :`B` 1.0 :`A` 1.0) 3.0))
    (:`Is Not Valid`
      (`KismetSystemLibrary.PrintString` "not valid" true true (struct :`G` 0.66 :`B` 1.0 :`A` 1.0) 3.0))))

(event `DebugAbilities`
  (bind _outabilityhandles (`AbilitySystemComponent.GetAllAbilities` (`self.AbilitySystemComponent`)))
  (for _array_element _outabilityhandles
    (`KismetSystemLibrary.PrintString` (`KismetSystemLibrary.GetDisplayName` (`.ReturnValue` (`AbilitySystemBlueprintLibrary.GetGameplayAbilityFromSpecHandle` (`self.AbilitySystemComponent`) _array_element))))))

(fn `GetPlayer`
  (returns (Player :type "/Game/_Main/Characters/BP_PlayerCharacter Object Reference"))
  (return null))

(fn `IsDead`
  (returns (Dead :type Boolean))
  (return false))

(fn `UpdateMovement`
  (params (CanMove :type Boolean))
  (returns (Return :type Boolean))
  (return false))

(fn `UserConstructionScript`)