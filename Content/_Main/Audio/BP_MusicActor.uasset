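; BP_MusicActor is a music player actor that plays an intro track followed by a loop track as non-spatialized 2D sound.
; BeginPlay packs the Intro and Loop sounds into a music struct and calls InitialiseSoundWave, which plays the intro.
; The Audio component's playback-percent event, gated by DoOnce, waits for the reported sound wave's duration before playing the loop track.
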(event `self.ReceiveBeginPlay`
  (`self.InitialiseSoundWave` (make `/Game/_Main/Audio/ST_MusicLoop` (`self.Intro`) (`self.Loop`))))

(event `InitialiseSoundWave`
  (params (MusicStruct :type "/Game/_Main/Audio/ST_MusicLoop Structure"))
  (`self.PlayFromStart`))

(event `self.Audio.OnAudioPlaybackPercent`
  (params (PlayingSoundWave :type "SoundWave Object Reference") (PlaybackPercent :type "Float (single-precision)"))
  (`/Engine/EditorBlueprintResources/StandardMacros.DoOnce` false
    (:`Completed`
      (`KismetSystemLibrary.Delay` (`SoundBase.Duration` PlayingSoundWave))
      (`self.PlayFromLoop`))))

(fn `PlayFromLoop`
  (`GameplayStatics.PlaySound2D` (`self.Loop`) 1.0 1.0 0.0 null null))

(fn `PlayFromStart`
  (`GameplayStatics.PlaySound2D` (`self.Intro`) 1.0 1.0 0.0 null null))

(fn `UserConstructionScript`)