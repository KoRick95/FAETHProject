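; BP_HealingCircle is a healing circle visual effect Blueprint that applies one configurable Colour across its Niagara effect and lights.
; The Colour variable drives the Colour parameter of NSHealingCircle and the light color of CharacterGlow and PulsingGlow.
; The construction script applies the tint and BeginPlay repeats it, with no other gameplay or healing logic in the graphs.
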(event `self.ReceiveBeginPlay`
  (`NiagaraComponent.SetVariableLinearColor` (`self.NS_HealingCircle`) "Colour" (`self.Colour`))
  (`LightComponent.SetLightColor` (`self.CharacterGlow`) (`self.Colour`) true)
  (`LightComponent.SetLightColor` (`self.PulsingGlow`) (`self.Colour`) true))

(fn `UserConstructionScript`
  (`NiagaraComponent.SetVariableLinearColor` (`self.NS_HealingCircle`) "Colour" (`self.Colour`))
  (`LightComponent.SetLightColor` (`self.CharacterGlow`) (`self.Colour`) true)
  (`LightComponent.SetLightColor` (`self.PulsingGlow`) (`self.Colour`) true))