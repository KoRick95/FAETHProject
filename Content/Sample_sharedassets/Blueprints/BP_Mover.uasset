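; BP_Mover is an actor that moves a referenced ActorToMove along its spline in a continuous loop.
; Each tick, if that actor is valid, it accumulates elapsed time and converts it, modulo RunTime, into a fraction of the spline's length.
; It then sets the actor's world location to that point, without sweep and without changing its rotation.
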(event `self.ReceiveTick`
  (params (DeltaSeconds :type "Float (single-precision)"))
  (bind _spline (`self.Spline`))
  (`/Engine/EditorBlueprintResources/StandardMacros.IsValid` (`self.Actor to move`)
    (:`Is Valid`
      (bind _output_get (set `self.Time running` (+ (`self.Time running`) DeltaSeconds)))
      (`self.K2_SetActorLocation` (`self.Actor to move`) (`SplineComponent.GetLocationAtDistanceAlongSpline` _spline (* (mod (/ _output_get (`self.Run time`)) 1.0) (`SplineComponent.GetSplineLength` _spline)) "World") false false))))

(fn `UserConstructionScript`)