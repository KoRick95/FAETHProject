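; Cel shading component that turns its owner's skeletal and static mesh materials into dynamic instances and feeds them scene lighting.
; Point and spot lights are cached in per-tick batches and periodically flagged for refresh.
; A looping timer bubble-sorts the cache by distance to the component.
; Another pushes the four leading lights' parameters into numbered material slots, along with the first directional light as the sun.
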(event `self.ReceiveBeginPlay`
  (bind _returnvalue (`self.GetOwner`))
  (bind _materials (`self.Materials`))
  (bind _fastlightupdaterate (`self.FastLightUpdateRate`))
  (`|ExecutionSequence` :!label _label
    (:`then_0`
      (`KismetSystemLibrary.K2_SetTimer` null "UpdateMaterials" _fastlightupdaterate true)
      (`KismetSystemLibrary.K2_SetTimer` null "FastSortLights" _fastlightupdaterate true)
      (`KismetSystemLibrary.K2_SetTimer` null "InvalidateLights" 60.0 true)
      (`self.GatherLights`)
      (`self.FastSortLights`)
      (`self.UpdateMaterials`))
    (:`then_1`
      ;[0 0 0] Find and configure components to cel shade
      (`|ExecutionSequence`
        (:`then_0`
          (for _array_element (`Actor.K2_GetComponentsByClass` _returnvalue "/Script/Engine.SkeletalMeshComponent")
            (for (_array_element_2 _array_index) (`MeshComponent.GetMaterials` _array_element)
              (bind _returnvalue_2 (`PrimitiveComponent.CreateDynamicMaterialInstance` _array_element _array_index _array_element_2 (`KismetStringLibrary.Conv_StringToName` (`KismetStringLibrary.Concat_StrStr` "CelMaterial" (`KismetStringLibrary.Conv_IntToString` _array_index)))))
              (`KismetArrayLibrary.Array_Add` _materials _returnvalue_2))))
        (:`then_1`
          (for _array_element_3 (`Actor.K2_GetComponentsByClass` _returnvalue "/Script/Engine.StaticMeshComponent")
            (for (_array_element_4 _array_index_2) (`MeshComponent.GetMaterials` _array_element_3)
              (bind _returnvalue_3 (`PrimitiveComponent.CreateDynamicMaterialInstance` _array_element_3 _array_index_2 _array_element_4 (`KismetStringLibrary.Conv_StringToName` (`KismetStringLibrary.Concat_StrStr` "CelMaterial" (`KismetStringLibrary.Conv_IntToString` _array_index_2)))))
              (`KismetArrayLibrary.Array_Add` _materials _returnvalue_3))))))))

(event `Construction`
  (goto _label))

(event `self.ReceiveTick`
  (params (DeltaSeconds :type "Float (single-precision)"))
  ;[0 0 0] Update lighting
  (`|ExecutionSequence`
    (:`then_0`
      (if (not (`self.DoneGathering`))
        (`self.GatherLights`)))))

(fn `FastSortLights`
  (locals (SortRange :type Integer) (Swapped :type Boolean :default true))
  (bind _lights (`self.Lights`))
  (`|ExecutionSequence`
    (:`then_0`
      (for _index (range (+ (`KismetArrayLibrary.Array_LastIndex` _lights) 1))
        (bind (_output_type _output_light _output_location _output_normal _output_distance) (break `/Game/Shaders/CelLightingModel/Blueprints/SCelLightDistance` (`|GetArrayItem` _lights _index)))
        (`|VariableSetRef` _output_distance (`KismetMathLibrary.VSize` (- (`self.K2_GetComponentLocation`) _output_location)))))
    (:`then_1`
      (set `local.SortRange` (- (`KismetArrayLibrary.Array_LastIndex` (`self.Lights`)) 1))
      (while (`local.Swapped`)
        (set `local.Swapped` false)
        (for _index_2 (range (+ (`local.SortRange`) 1))
          (bind _returnvalue (+ _index_2 1))
          (bind (_output_type_2 _output_light_2 _output_location_2 _output_normal_2 _output_distance_2) (break `/Game/Shaders/CelLightingModel/Blueprints/SCelLightDistance` (`|GetArrayItem` (`self.Lights`) _returnvalue)))
          (bind (_output_type_3 _output_light_3 _output_location_3 _output_normal_3 _output_distance_3) (break `/Game/Shaders/CelLightingModel/Blueprints/SCelLightDistance` (`|GetArrayItem` (`self.Lights`) _index_2)))
          (if (< _output_distance_2 _output_distance_3)
            (`KismetArrayLibrary.Array_Swap` (`self.Lights`) _index_2 _returnvalue)
            (set `local.Swapped` true)))))))

(fn `FindLight`
  (params (Light :type "LightComponent Object Reference"))
  (returns (Index :type Integer) (Distance :type "Float (double-precision)") (ReadyToInvalidate :type Boolean) (Success :type Boolean))
  (for (_array_element _array_index) (`self.Lights`)
    (if (== (`.Light_14_B37FAE7F4BD9942DCABFF39975485097` (break `/Game/Shaders/CelLightingModel/Blueprints/SCelLightDistance` _array_element)) Light)
      (return _array_index (`.Distance_5_09A1DA654A29670143223E811BAEAFD7` (break `/Game/Shaders/CelLightingModel/Blueprints/SCelLightDistance` _array_element)) (`.ReadyToInvalidate_10_AAA2D2FE4D92E0C641A684B58458C9D4` (break `/Game/Shaders/CelLightingModel/Blueprints/SCelLightDistance` _array_element)) true)))
  (return 0 0.0 true false))

(fn `FindLightByDistance`
  (params (CelLightAndDistance :type "/Game/Shaders/CelLightingModel/Blueprints/SCelLightDistance Structure"))
  (returns (Index :type Integer))
  (bind _lights (`self.Lights`))
  (for (_array_element _array_index) _lights
    (if (< CelLightAndDistance_Distance_5_09A1DA654A29670143223E811BAEAFD7 (`.Distance_5_09A1DA654A29670143223E811BAEAFD7` (break `/Game/Shaders/CelLightingModel/Blueprints/SCelLightDistance` _array_element)))
      (return _array_index)))
  (return (`KismetArrayLibrary.Array_Length` _lights)))

(fn `GatherLights`
  (locals (LocalLights :type "Array of /Game/Shaders/CelLightingModel/Blueprints/SCelLightDistance Structure") (LightsHandled :type Integer) (FirstRun :type Boolean :default false))
  (bind _lights (`self.Lights`))
  (bind _lights_2 (`self.Lights`))
  (set `local.LightsHandled` 0)
  (`|ExecutionSequence`
    (:`then_0`
      (bind _outactors (`GameplayStatics.GetAllActorsOfClass` "/Script/Engine.PointLight"))
      (for _array_element _outactors
        (bind (_index _distance _readytoinvalidate _success) (`self.FindLight` (`PointLight.PointLightComponent` _array_element)))
        (if (and (or _readytoinvalidate (not _success)) (< (`local.LightsHandled`) (`self.Lights To Gather Per Tick`)))
          (if (`self.IsVisible` (`PointLight.PointLightComponent` _array_element))
            (`/Engine/EditorBlueprintResources/StandardMacros.IncrementInt` (`local.LightsHandled`)
              (:`  `
                (if (not _success)
                  (bind _returnvalue (`Actor.K2_GetActorLocation` _array_element))
                  (bind _scellightdistance (make `/Game/Shaders/CelLightingModel/Blueprints/SCelLightDistance` "NewEnumerator0" (`PointLight.PointLightComponent` _array_element) _returnvalue (0.0 0.0 0.0) (`KismetMathLibrary.VSize` (- (`self.K2_GetComponentLocation`) _returnvalue)) 0.0 0.0 false))
                  (`KismetArrayLibrary.Array_Add` _lights_2 _scellightdistance)
                  (else
                    (`KismetArrayLibrary.Array_Set` _lights_2 _index _scellightdistance)))))))))
    (:`then_1`
      (bind _outactors_2 (`GameplayStatics.GetAllActorsOfClass` "/Script/Engine.SpotLight"))
      (for _array_element_2 _outactors_2
        (bind _lightcomponent (`Light.LightComponent` _array_element_2))
        (bind (_index_2 _distance_2 _readytoinvalidate_2 _success_2) (`self.FindLight` _lightcomponent))
        (if (and (or _readytoinvalidate_2 (not _success_2)) (< (`local.LightsHandled`) (`self.Lights To Gather Per Tick`)))
          (if (`self.IsVisible` _lightcomponent)
            (`/Engine/EditorBlueprintResources/StandardMacros.IncrementInt` (`local.LightsHandled`)
              (:`  `
                (if (not _success_2)
                  (bind _returnvalue_2 (`Actor.K2_GetActorLocation` _array_element_2))
                  (bind _spotlightcomponent (`SpotLight.SpotLightComponent` _array_element_2))
                  (bind _scellightdistance_2 (make `/Game/Shaders/CelLightingModel/Blueprints/SCelLightDistance` "NewEnumerator1" _lightcomponent _returnvalue_2 (`self.GetForwardVector` _lightcomponent) (`KismetMathLibrary.VSize` (- (`self.K2_GetComponentLocation`) _returnvalue_2)) (`SpotLightComponent.InnerConeAngle` _spotlightcomponent) (`SpotLightComponent.OuterConeAngle` _spotlightcomponent) false))
                  (`KismetArrayLibrary.Array_Add` _lights _scellightdistance_2)
                  (else
                    (`KismetArrayLibrary.Array_Set` _lights _index_2 _scellightdistance_2)))))))))
    (:`then_2`
      (set `self.DoneGathering` (== (`local.LightsHandled`) 0))
      (`self.FastSortLights`))))

(fn `InvalidateLights`
  (bind _lights (`self.Lights`))
  (for (_ _array_index) _lights
    (bind (_output_type _output_light _output_location _output_normal _output_distance _output_inner _output_outer _output_readytoinvalidate) (break `/Game/Shaders/CelLightingModel/Blueprints/SCelLightDistance` (`|GetArrayItem` _lights _array_index)))
    (`|VariableSetRef` _output_readytoinvalidate true)
    (set `self.DoneGathering` false)))

(fn `RemoveLight`
  (params (Light :type "LightComponent Object Reference"))
  (bind (_index _distance _readytoinvalidate _success) (`self.FindLight` Light))
  (if _success
    (`KismetArrayLibrary.Array_Remove` (`self.Lights`) _index)))

(fn `SetMaterialParameters`
  (params (Material :type "MaterialInstanceDynamic Object Reference") (Index :type Integer) (Parameters :type "/Game/Shaders/CelLightingModel/Blueprints/SLightAverage Structure"))
  (bind _returnvalue (`KismetStringLibrary.Conv_IntToString` Index))
  (`|ExecutionSequence`
    (:`then_0`
      (`MaterialInstanceDynamic.SetVectorParameterValue` Material (`KismetStringLibrary.Conv_StringToName` (`KismetStringLibrary.Concat_StrStr` "LightColour" _returnvalue)) (`KismetMathLibrary.Conv_VectorToLinearColor` Parameters_Colour_13_17227BAF4A09921934A6048932A3D148)))
    (:`then_1`
      (`MaterialInstanceDynamic.SetVectorParameterValue` Material (`KismetStringLibrary.Conv_StringToName` (`KismetStringLibrary.Concat_StrStr` "LightPosition" _returnvalue)) (`KismetMathLibrary.Conv_VectorToLinearColor` Parameters_Position_7_7B4D9442447514D13A3E159D972F4410)))
    (:`then_2`
      (`MaterialInstanceDynamic.SetScalarParameterValue` Material (`KismetStringLibrary.Conv_StringToName` (`KismetStringLibrary.Concat_StrStr` "LightAttenuation" _returnvalue)) Parameters_Attenuation_10_C56EBD32449CABD8C93FC6A87958E3BC))
    (:`then_3`
      (`MaterialInstanceDynamic.SetScalarParameterValue` Material (`KismetStringLibrary.Conv_StringToName` (`KismetStringLibrary.Concat_StrStr` "LightIntensity" _returnvalue)) Parameters_Intensity_12_0931C6CC407B1034530E66B788E0F3A0))
    (:`then_4`
      (`MaterialInstanceDynamic.SetVectorParameterValue` Material (`KismetStringLibrary.Conv_StringToName` (`KismetStringLibrary.Concat_StrStr` "Normal" _returnvalue)) (`KismetMathLibrary.Conv_VectorToLinearColor` Parameters_Normal_21_69C7906E4A3626C62E29B39FE1AFBE4B)))
    (:`then_5`
      (`MaterialInstanceDynamic.SetScalarParameterValue` Material (`KismetStringLibrary.Conv_StringToName` (`KismetStringLibrary.Concat_StrStr` "InnerCone" _returnvalue)) Parameters_Inner_16_3D11EA4540D42081C8CCB1B18A959DFB))
    (:`then_6`
      (`MaterialInstanceDynamic.SetScalarParameterValue` Material (`KismetStringLibrary.Conv_StringToName` (`KismetStringLibrary.Concat_StrStr` "OuterCone" _returnvalue)) Parameters_Outer_18_DD0A82844D6FD3BD454D4EAA32E4A685))
    (:`then_7`
      (`MaterialInstanceDynamic.SetScalarParameterValue` Material (`KismetStringLibrary.Conv_StringToName` (`KismetStringLibrary.Concat_StrStr` "LightType" _returnvalue)) (`KismetMathLibrary.Conv_ByteToDouble` Parameters_Type_24_7164E65147B9A0434CE8FCAE68964F4D)))))

(fn `UpdateLightAverages`
  (locals (LocalLightAverage :type "/Game/Shaders/CelLightingModel/Blueprints/SLightAverage Structure"))
  (bind _lights (`self.Lights`))
  (if (> (`KismetArrayLibrary.Array_Length` _lights) 0)
    (for _index (range (+ (`KismetMathLibrary.Min` (`KismetArrayLibrary.Array_LastIndex` _lights) 3) 1))
      (`|ExecutionSequence`
        (:`then_0`
          (bind (_output_type _output_colour _output_position _output_intensity _output_attenuation _output_inner _output_outer _output_normal) (break `/Game/Shaders/CelLightingModel/Blueprints/SLightAverage` (`|GetArrayItem` (`self.LightArray`) _index)))
          (bind (_output_type_2 _output_light) (break `/Game/Shaders/CelLightingModel/Blueprints/SCelLightDistance` (`|GetArrayItem` (`self.Lights`) _index)))
          (`|VariableSetRef` _output_colour (`KismetMathLibrary.Conv_LinearColorToVector` (`LightComponentBase.GetLightColor` _output_light))))
        (:`then_1`
          (`|VariableSetRef` _output_position (`self.K2_GetComponentLocation` _output_light)))
        (:`then_2`
          (`|VariableSetRef` _output_intensity (`LightComponentBase.Intensity` _output_light)))
        (:`then_3`
          (if (`|EnumEquality` _output_type_2 "NewEnumerator0")
            (bind _aspoint_light_component (cast `PointLightComponent` _output_light))
            (`|VariableSetRef` _output_attenuation (`LocalLightComponent.AttenuationRadius` _aspoint_light_component))
            (`|VariableSetRef` _output_type "NewEnumerator0")))
        (:`then_4`
          (if (`|EnumEquality` _output_type_2 "NewEnumerator1")
            (bind _asspot_light_component (cast `SpotLightComponent` _output_light))
            (`|ExecutionSequence`
              (:`then_0`
                (`|VariableSetRef` _output_inner (`SpotLightComponent.InnerConeAngle` _asspot_light_component))
                (`|VariableSetRef` _output_type "NewEnumerator1"))
              (:`then_1`
                (`|VariableSetRef` _output_outer (`SpotLightComponent.OuterConeAngle` _asspot_light_component)))
              (:`then_2`
                (`|VariableSetRef` _output_normal (`self.GetForwardVector` _asspot_light_component)))
              (:`then_3`
                (`|VariableSetRef` _output_attenuation (`LocalLightComponent.AttenuationRadius` _asspot_light_component))))))))))

(fn `UpdateMaterials`
  (`self.UpdateLightAverages`)
  (for _array_element (`self.Materials`)
    (`|ExecutionSequence`
      (:`then_0`
        (if (`KismetMathLibrary.Conv_IntToBool` (`KismetArrayLibrary.Array_Length` (`self.Lights`)))
          (for _index (range (+ (`KismetMathLibrary.Min` (`KismetArrayLibrary.Array_LastIndex` (`self.LightArray`)) 3) 1))
            (`self.SetMaterialParameters` _array_element (+ _index 1) (`|GetArrayItem` (`self.LightArray`) _index)))))
      (:`then_1`
        (bind _outactors (`GameplayStatics.GetAllActorsOfClass` "/Script/Engine.DirectionalLight"))
        ;[1 1 1] Fix the Cel thing
        (if (> (`KismetArrayLibrary.Array_Length` _outactors) 0)
          (bind _output (`|GetArrayItem` _outactors))
          (`/Engine/EditorBlueprintResources/StandardMacros.IsValid` _output
            (:`Is Valid`
              (bind _lightcomponent (`Light.LightComponent` _output))
              (`MaterialInstanceDynamic.SetVectorParameterValue` _array_element "SunColour" (`LightComponentBase.GetLightColor` _lightcomponent))
              (`MaterialInstanceDynamic.SetVectorParameterValue` _array_element "SunDirection" (`KismetMathLibrary.Conv_VectorToLinearColor` (`KismetMathLibrary.BreakRotIntoAxes` (`self.K2_GetComponentRotation` _lightcomponent))))
              (`MaterialInstanceDynamic.SetScalarParameterValue` _array_element "SunIntensity" (`LightComponentBase.Intensity` _lightcomponent)))))))))